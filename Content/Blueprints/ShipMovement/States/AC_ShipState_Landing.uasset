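; Ship movement state that handles landing at the controller's target station.
; On enter, it has the station build a landing track from the ship's current location, then makes that the controller's current spline, starting at zero distance, moving forward.
; Each tick delegates movement along the spline to the ship controller.
; On exit, it records itself as the previous state and marks the ship as at the target station.
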(event `/Game/Blueprints/ShipMovement/States/BPI_ShipState.OnEnter`
  (params (ACShipController :type "/Game/Blueprints/ShipMovement/AC_ShipController Object Reference"))
  (bind _acship_controller (`self.ACShip Controller`))
  (bind _acship_controller_2 (`self.ACShip Controller`))
  (bind _targetstation (`/Game/Blueprints/ShipMovement/AC_ShipController.TargetStation` _acship_controller))
  (bind _output_get (set `self.ACShip Controller` ACShipController))
  (set `/Game/Blueprints/ShipMovement/AC_ShipController.State` "NewEnumerator3" _output_get)
  (`/Game/Blueprints/BP_Station.SetLandingTrack` _targetstation (`Actor.K2_GetActorLocation` (`/Game/Blueprints/ShipMovement/AC_ShipController.ShipActor` _acship_controller)))
  (set `/Game/Blueprints/ShipMovement/AC_ShipController.CurrentSpline` (`/Game/Blueprints/BP_Station.LandingTrack` _targetstation) _acship_controller_2)
  (set `/Game/Blueprints/ShipMovement/AC_ShipController.DistanceAlongSpline` 0.0 _acship_controller_2)
  (set `/Game/Blueprints/ShipMovement/AC_ShipController.IsForwardOnCurrentSpline` true _acship_controller_2))

(event `/Game/Blueprints/ShipMovement/States/BPI_ShipState.Tick`
  (params (ACShipController :type "/Game/Blueprints/ShipMovement/AC_ShipController Object Reference"))
  (`/Game/Blueprints/ShipMovement/AC_ShipController.MoveAlongCurrentSpline` ACShipController false))

(event `/Game/Blueprints/ShipMovement/States/BPI_ShipState.OnExit`
  (params (ACShipController :type "/Game/Blueprints/ShipMovement/AC_ShipController Object Reference"))
  (set `/Game/Blueprints/ShipMovement/AC_ShipController.PrevState` "NewEnumerator3" ACShipController)
  (set `/Game/Blueprints/ShipMovement/AC_ShipController.AtStation` (`/Game/Blueprints/ShipMovement/AC_ShipController.TargetStation` ACShipController) ACShipController))