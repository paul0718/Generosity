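; Ship movement state component that handles docking at the target station.
; On enter it switches the ship controller onto the station's docking track spline from the start.
; Each tick it first rotates the ship horizontally to the dock's world yaw, then moves it along that spline once aligned.
; On exit it records itself as the previous state and marks the target station as the one the ship is at.
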(event `/Game/Blueprints/ShipMovement/States/BPI_ShipState.OnEnter`
  (params (ACShipController :type "/Game/Blueprints/ShipMovement/AC_ShipController Object Reference"))
  (set `/Game/Blueprints/ShipMovement/AC_ShipController.State` "NewEnumerator4" ACShipController)
  (set `self.isPostureReady` false)
  (`/Game/Blueprints/ShipMovement/AC_ShipController.SwitchToSpline` ACShipController (`/Game/Blueprints/BP_Station.DockingTrack` (`/Game/Blueprints/ShipMovement/AC_ShipController.TargetStation` ACShipController)) true 0.0))

(event `/Game/Blueprints/ShipMovement/States/BPI_ShipState.Tick`
  (params (ACShipController :type "/Game/Blueprints/ShipMovement/AC_ShipController Object Reference"))
  (bind (_returnvalue_roll _returnvalue_pitch _returnvalue_yaw) (`KismetMathLibrary.BreakRotator` (`SceneComponent.K2_GetComponentRotation` (`/Game/Blueprints/BP_Station.Dock` (`/Game/Blueprints/ShipMovement/AC_ShipController.TargetStation` ACShipController)))))
  (if (`self.isPostureReady`)
    (`/Game/Blueprints/ShipMovement/AC_ShipController.MoveAlongCurrentSpline` ACShipController false)
    (else
      (bind _rotationdone (`/Game/Blueprints/ShipMovement/AC_ShipController.RotateHorizontalTowardsWorld` ACShipController _returnvalue_yaw))
      (set `self.isPostureReady` _rotationdone))))

(event `/Game/Blueprints/ShipMovement/States/BPI_ShipState.OnExit`
  (params (ACShipController :type "/Game/Blueprints/ShipMovement/AC_ShipController Object Reference"))
  (set `/Game/Blueprints/ShipMovement/AC_ShipController.PrevState` "NewEnumerator4" ACShipController)
  (set `/Game/Blueprints/ShipMovement/AC_ShipController.AtStation` (`/Game/Blueprints/ShipMovement/AC_ShipController.TargetStation` ACShipController) ACShipController))