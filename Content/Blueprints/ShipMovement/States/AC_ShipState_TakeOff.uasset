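; Ship movement state for taking off from a station back onto its current line, expected between two OnLine states.
; On enter it picks an attach point just past the station along the line direction and shapes the station's take-off track to meet it.
; Tick turns the ship to the line's yaw at that point before moving it along the track.
; On exit it hands the ship to the line spline at the attach point.
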(event `/Game/Blueprints/ShipMovement/States/BPI_ShipState.OnEnter`
  (params (ACShipController :type "/Game/Blueprints/ShipMovement/AC_ShipController Object Reference"))
  (bind _acship_controller (`self.ACShip Controller`))
  (bind _acship_controller_2 (`self.ACShip Controller`))
  (bind _atstation (`/Game/Blueprints/ShipMovement/AC_ShipController.AtStation` _acship_controller_2))
  (bind _spline (`/Game/Blueprints/BP_Spline_Road.Spline` (`/Game/Blueprints/ShipMovement/AC_ShipController.CurrentLine` _acship_controller_2)))
  ;[1 1 1] Previous State Must Be OnLine
  (bind _output_get (set `self.ACShip Controller` ACShipController))
  (set `/Game/Blueprints/ShipMovement/AC_ShipController.State` "NewEnumerator2" _output_get)
  (set `self.isPostureReady` false)
  (bind _currlinedirection (`/Game/Blueprints/ShipMovement/AC_ShipController.GetCurrLineDirection` _acship_controller))
  (bind _output_get_2 (set `self.AttachPointInputKey` (+ (`BlueprintMapLibrary.Map_Find` (`/Game/Blueprints/BP_Station.InputKeysOnLines` (`/Game/Blueprints/ShipMovement/AC_ShipController.AtStation` _acship_controller)) (`/Game/Blueprints/ShipMovement/AC_ShipController.CurrentLineIndex` _acship_controller)) (* 0.25 _currlinedirection))))
  (bind _returnvalue (`SplineComponent.GetTransformAtSplineInputKey` _spline _output_get_2 "World" false))
  (set `self.TargetRotationZWorld` (.yaw (.rotation _returnvalue)))
  (`/Game/Blueprints/BP_Station.SetTakeOffTrack` _atstation (.location _returnvalue) (* (`SplineComponent.GetTangentAtSplineInputKey` _spline _output_get_2 "World") 0.5))
  (`/Game/Blueprints/ShipMovement/AC_ShipController.SwitchToSpline` (`self.ACShip Controller`) (`/Game/Blueprints/BP_Station.TakeOffTrack` _atstation) true 0.0))

(event `/Game/Blueprints/ShipMovement/States/BPI_ShipState.Tick`
  (params (ACShipController :type "/Game/Blueprints/ShipMovement/AC_ShipController Object Reference"))
  (if (`self.isPostureReady`)
    (`/Game/Blueprints/ShipMovement/AC_ShipController.MoveAlongCurrentSpline` ACShipController false)
    (else
      (bind _rotationdone (`/Game/Blueprints/ShipMovement/AC_ShipController.RotateHorizontalTowardsWorld` ACShipController (`self.TargetRotationZWorld`)))
      (set `self.isPostureReady` _rotationdone))))

(event `/Game/Blueprints/ShipMovement/States/BPI_ShipState.OnExit`
  (params (ACShipController :type "/Game/Blueprints/ShipMovement/AC_ShipController Object Reference"))
  (bind _acship_controller (`self.ACShip Controller`))
  (bind _spline (`/Game/Blueprints/BP_Spline_Road.Spline` (`/Game/Blueprints/ShipMovement/AC_ShipController.CurrentLine` ACShipController)))
  ;[1 1 1] Next State Must Be OnLine
  (set `/Game/Blueprints/ShipMovement/AC_ShipController.CurrentSpline` _spline ACShipController)
  (set `/Game/Blueprints/ShipMovement/AC_ShipController.DistanceAlongSpline` (`SplineComponent.GetDistanceAlongSplineAtSplineInputKey` _spline (`self.AttachPointInputKey`)) _acship_controller)
  (set `/Game/Blueprints/ShipMovement/AC_ShipController.IsForwardOnCurrentSpline` (`/Game/Blueprints/ShipMovement/AC_ShipController.IsForwardOnLine` _acship_controller) _acship_controller)
  (set `/Game/Blueprints/ShipMovement/AC_ShipController.PrevState` "NewEnumerator2" _acship_controller))