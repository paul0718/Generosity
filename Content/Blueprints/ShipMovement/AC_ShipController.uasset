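; Ship controller component that moves its owning ship along splines between stations from BP_NaviSystem.
; A state machine of components added at BeginPlay runs Undocking, Take Off, On Line, Landing, Docking and Stopped, each handling enter, tick and exit.
; Tick switches states at spline ends, or to Landing near the target station's spline input key.
; Shared helpers handle reversible, loop-aware spline movement, turning and spline switching, alongside test keys and a docked-start setup.
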(event `Key|Up`
  (params (Key :type "Key Structure"))
  ;[1 1 1] Reverse On Track
  (:`Pressed`
    (`/Engine/EditorBlueprintResources/StandardMacros.FlipFlop`
      (:`A`
        (set `self.IsForwardOnCurrentSpline` false))
      (:`B`
        (set `self.IsForwardOnCurrentSpline` true)))))

(event `Key|Equals`
  (params (Key :type "Key Structure"))
  ;[1 1 1] State Machine Testing
  (:`Pressed`
    (`self.UpdateState` (`self.StateUndocking`))))

(event `self.ReceiveBeginPlay`
  (bind _shipactor (`self.ShipActor`))
  (bind _shipactor_2 (`self.ShipActor`))
  (bind (_returnvalue_roll _returnvalue_pitch) (`KismetMathLibrary.BreakRotator` (`Actor.K2_GetActorRotation` _shipactor)))
  (bind _dock (`/Game/Blueprints/BP_Station.Dock` (`self.AtStation`)))
  (bind (_returnvalue_roll_2 _returnvalue_pitch_2 _returnvalue_yaw) (`KismetMathLibrary.BreakRotator` (`SceneComponent.K2_GetComponentRotation` _dock)))
  (bind _returnvalue (`GameplayStatics.GetActorOfClass` "/Game/Blueprints/BP_NaviSystem.BP_NaviSystem_C"))
  (set `self.NaviSystem` _returnvalue)
  (set `self.CurrentSpline` (`/Game/Blueprints/BP_Spline_Road.Spline` (`self.CurrentLine`)))
  (bind _output_get (set `self.ShipActor` (`self.GetOwner`)))
  (set `self.InitialWorldRotation` (`Actor.K2_GetActorRotation` _output_get))
  (`|ExecutionSequence`
    (:`then_0`
      (bind _returnvalue_2 (`|AddComponentByClass` _shipactor_2 "/Game/Blueprints/ShipMovement/States/AC_ShipState_Stopped.AC_ShipState_Stopped_C"))
      (set `self.StateStopped` _returnvalue_2))
    (:`then_1`
      (bind _returnvalue_3 (`|AddComponentByClass` _shipactor_2 "/Game/Blueprints/ShipMovement/States/AC_ShipState_OnLine.AC_ShipState_OnLine_C"))
      (set `self.StateOnLine` _returnvalue_3))
    (:`then_2`
      (bind _returnvalue_4 (`|AddComponentByClass` _shipactor_2 "/Game/Blueprints/ShipMovement/States/AC_ShipState_TakeOff.AC_ShipState_TakeOff_C"))
      (set `self.StateTakeOff` _returnvalue_4))
    (:`then_3`
      (bind _returnvalue_5 (`|AddComponentByClass` _shipactor_2 "/Game/Blueprints/ShipMovement/States/AC_ShipState_Landing.AC_ShipState_Landing_C"))
      (set `self.StateLanding` _returnvalue_5))
    (:`then_4`
      (bind _returnvalue_6 (`|AddComponentByClass` _shipactor_2 "/Game/Blueprints/ShipMovement/States/AC_ShipState_Docking.AC_ShipState_Docking_C"))
      (set `self.StateDocking` _returnvalue_6))
    (:`then_5`
      (bind _returnvalue_7 (`|AddComponentByClass` _shipactor_2 "/Game/Blueprints/ShipMovement/States/AC_ShipState_Undocking.AC_ShipState_Undocking_C"))
      (set `self.StateUndocking` _returnvalue_7))
    (:`then_7`
      (set `self.CurrentStateInstance` (`self.StateStopped`)))
    (:`then_8`
      ;[1 1 1] Need to setup after stations setup
      (`KismetSystemLibrary.Delay` 0.5)
      ;[1 1 1] For Testing, Assume stopped at a station
      (`Actor.K2_SetActorLocation` (`self.ShipActor`) (`SceneComponent.K2_GetComponentLocation` _dock) false false)
      (`Actor.K2_SetActorRotation` _shipactor (`KismetMathLibrary.MakeRotator` _returnvalue_roll _returnvalue_pitch (+ _returnvalue_yaw 180.0)) false))))

(event `self.ReceiveTick`
  (params (DeltaSeconds :type "Float (single-precision)"))
  (bind _returnvalue (`SplineComponent.GetInputKeyValueAtDistanceAlongSpline` (`self.CurrentSpline`) (`self.DistanceAlongSpline`)))
  (`|ExecutionSequence`
    (:`then_0`
      (switch `/Game/Blueprints/ShipMovement/States/EM_ShipState` (`self.State`)
        (:`NewEnumerator1`
          (`|ExecutionSequence`
            (:`then_0`
              (bind _hasreachedendofspline (`self.HasReachedEndOfSpline`))
              (if _hasreachedendofspline
                ;[1 1 1] TODO: change to steer state
                (`self.UpdateState` (`self.StateStopped`))))
            (:`then_1`
              ;[1 1 1] Close enough to target station?
              (if (<= (`KismetMathLibrary.Abs` (- (`BlueprintMapLibrary.Map_Find` (`/Game/Blueprints/BP_Station.InputKeysOnLines` (`self.TargetStation`)) (`self.CurrentLineIndex`)) _returnvalue)) 0.25)
                (`self.UpdateState` (`self.StateLanding`))))))
        (:`NewEnumerator2`
          (bind _hasreachedendofspline_2 (`self.HasReachedEndOfSpline`))
          (if _hasreachedendofspline_2
            (`self.UpdateState` (`self.StateOnLine`))))
        (:`NewEnumerator3`
          (bind _hasreachedendofspline_3 (`self.HasReachedEndOfSpline`))
          (if _hasreachedendofspline_3
            (`self.UpdateState` (`self.StateDocking`))))
        (:`NewEnumerator4`
          (bind _hasreachedendofspline_4 (`self.HasReachedEndOfSpline`))
          (if _hasreachedendofspline_4
            (`self.UpdateState` (`self.StateStopped`))))
        (:`NewEnumerator5`
          (bind _hasreachedendofspline_5 (`self.HasReachedEndOfSpline`))
          (if _hasreachedendofspline_5
            (`self.UpdateState` (`self.StateTakeOff`))))))
    (:`then_1`
      (`/Game/Blueprints/ShipMovement/States/AC_Abstract_ShipState.Tick` (`self.CurrentStateInstance`) self))
    (:`then_2`
      (`KismetSystemLibrary.PrintText` (`KismetTextLibrary.Conv_DoubleToText` _returnvalue "HalfToEven") true true (struct :`G` 0.66 :`B` 1.0 :`A` 1.0) 2.0 "0"))))

(fn `GetCurrLineDirection`
  (returns (CurrLineDirection :type Integer))
  (return (`KismetMathLibrary.FTrunc` (- (* (`KismetMathLibrary.Conv_BoolToDouble` (`self.IsForwardOnLine`)) 2.0) 1.0))))

(fn `GetCurrSplineDirection`
  (returns (ReturnValue :type Integer))
  (return (`KismetMathLibrary.FTrunc` (- (* (`KismetMathLibrary.Conv_BoolToDouble` (`self.IsForwardOnCurrentSpline`)) 2.0) 1.0))))

(fn `HasReachedEndOfSpline`
  (returns (HasReachedEndOfSpline :type Boolean))
  (`|ExecutionSequence`
    (:`then_0`
      (if (`SplineComponent.IsClosedLoop` (`self.CurrentSpline`))
        (return false)))
    (:`then_1`
      (if (`self.IsForwardOnCurrentSpline`)
        (return (== (`self.DistanceAlongSpline`) (`SplineComponent.GetSplineLength` (`self.CurrentSpline`))))
        (else
          (return (== (`self.DistanceAlongSpline`) 0.0)))))))

(fn `MoveAlongCurrentSpline`
  (params (changeRotation :type Boolean :default true))
  (bind (_initialworldrotation_roll _initialworldrotation_pitch _initialworldrotation_yaw) (`KismetMathLibrary.BreakRotator` (`self.InitialWorldRotation`)))
  (bind _currentspline (`self.CurrentSpline`))
  (bind _returnvalue (`SplineComponent.GetSplineLength` _currentspline))
  (bind _output_get (set `self.DistanceAlongSpline` (+ (* (* (`GameplayStatics.GetWorldDeltaSeconds`) (`self.Speed`)) (`self.FwdBwd`)) (`self.DistanceAlongSpline`))))
  ;[1 1 1] move (and rotate if needed) based on spline and direction on spline
  (`Actor.K2_SetActorLocation` (`self.ShipActor`) (`SplineComponent.GetLocationAtDistanceAlongSpline` (`self.CurrentSpline`) _output_get "World") false false)
  (if (`local.changeRotation`)
    (bind (_returnvalue_roll _returnvalue_pitch _returnvalue_yaw) (`KismetMathLibrary.BreakRotator` (`SplineComponent.GetRotationAtDistanceAlongSpline` (`self.CurrentSpline`) _output_get "World")))
    (`Actor.K2_SetActorRotation` (`self.ShipActor`) (`KismetMathLibrary.MakeRotator` _initialworldrotation_roll _initialworldrotation_pitch (- (+ (+ _initialworldrotation_yaw _returnvalue_yaw) (* (- 1.0 (`KismetMathLibrary.Conv_BoolToDouble` (`self.IsForwardOnCurrentSpline`))) 180.0)) 180.0)) false))
  ;[1 1 1] Clamp to [0, length] so it works on loops and reverse directions
  (if (`SplineComponent.IsClosedLoop` _currentspline)
    (set `self.DistanceAlongSpline` (mod (+ (mod _output_get _returnvalue) _returnvalue) _returnvalue))
    (else
      (set `self.DistanceAlongSpline` (`KismetMathLibrary.FClamp` _output_get 0.0 _returnvalue)))))

(fn `RotateHorizontalTowardsWorld`
  (params (TargetZ :type "Float (double-precision)"))
  (returns (RotationDone :type Boolean))
  (locals (TargetRotator :type "Rotator Structure") (CurrentRotator :type "Rotator Structure"))
  (bind _targetrotator (`local.TargetRotator`))
  (bind _returnvalue (`KismetMathLibrary.RInterpTo` (`local.CurrentRotator`) _targetrotator (`GameplayStatics.GetWorldDeltaSeconds`) (`self.DegPerSec`)))
  (bind _output_get (set `local.CurrentRotator` (`Actor.K2_GetActorRotation` (`self.ShipActor`))))
  (set `local.TargetRotator` (`KismetMathLibrary.MakeRotator` (.roll _output_get) (.pitch _output_get) (+ TargetZ 180.0)))
  (if (== (`local.CurrentRotator`) (`local.TargetRotator`) :`ErrorTolerance` 0.1)
    (return true)
    (else
      (`Actor.K2_SetActorRotation` (`self.ShipActor`) _returnvalue false)
      (if (== _returnvalue _targetrotator :`ErrorTolerance` 0.1)
        (return true)
        (else
          (return false))))))

(fn `Set Destination`
  (params (`Station Name` :type Name))
  (bind (_value _returnvalue) (`BlueprintMapLibrary.Map_Find` (`/Game/Blueprints/BP_NaviSystem.Stations` (`self.NaviSystem`)) `Station Name`))
  (if _returnvalue
    (set `self.TargetStation` _value)
    (else
      (`KismetSystemLibrary.PrintText` "ShipController::SetDestination: Station Not Found"))))

(fn `SwitchToSpline`
  (params (NewSpline :type "SplineComponent Object Reference") (isForwardOnNewSpline :type Boolean) (startDistanceAlongNewSpline :type "Float (double-precision)"))
  ;[1 1 1] Ship At Switch Location?
  (if (== (`SplineComponent.GetLocationAtDistanceAlongSpline` NewSpline startDistanceAlongNewSpline "World") (`Actor.K2_GetActorLocation` (`self.ShipActor`)) :`ErrorTolerance` 0.01)
    (set `self.CurrentSpline` (`local.NewSpline`))
    (set `self.IsForwardOnCurrentSpline` (`local.isForwardOnNewSpline`))
    (set `self.DistanceAlongSpline` (`local.startDistanceAlongNewSpline`))
    (else
      (`KismetSystemLibrary.PrintText` "AC_ShipController::SwitchToSpline: Ship not at switch location"))))

(fn `UpdateState`
  (params (NewStateInstance :type "/Game/Blueprints/ShipMovement/States/AC_Abstract_ShipState Object Reference"))
  (`|ExecutionSequence`
    (:`then_0`
      (`/Game/Blueprints/ShipMovement/States/BPI_ShipState.OnExit` (`self.CurrentStateInstance`) self))
    (:`then_1`
      (bind _output_get (set `self.CurrentStateInstance` NewStateInstance))
      (`/Game/Blueprints/ShipMovement/States/BPI_ShipState.OnEnter` _output_get self))))