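; Inventory component that stores cargo in fixed spots on the Shelf of its BP_QuarterBase owner.
; On BeginPlay it spawns and attaches a BI_CargoPlaceholder at each owner-relative cargo spot to fill the inventory list.
; Adding cargo swaps it into the first empty slot, caches that placeholder and reports whether it fit.
; Removing cargo disables it and moves a cached placeholder back into its slot and transform.
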(event `self.ReceiveBeginPlay`
  (for _array_element (`self.CargoSpots`)
    (bind _returnvalue (`|SpawnActorFromClass` "/Game/Blueprints/BI_CargoPlaceholder.BI_CargoPlaceholder_C" (`KismetMathLibrary.ComposeTransforms` _array_element (`Actor.GetTransform` (`self.GetOwner`))) "Undefined" "MultiplyWithRoot" (`self.GetOwner`) null))
    (bind _asbp_quarter_base (cast `/Game/Blueprints/BP_QuarterBase` (`self.GetOwner`)))
    (`Actor.K2_AttachToComponent` _returnvalue (`/Game/Blueprints/BP_QuarterBase.Shelf` _asbp_quarter_base) "None" "KeepWorld" "KeepWorld" "KeepWorld" true)
    (`KismetArrayLibrary.Array_Add` (`self.InventoryList`) _returnvalue))
  (set `self.InventorySize` (`KismetArrayLibrary.Array_Length` (`self.CargoSpots`))))

(fn `AddCargoAtNextAvailbleSpot`
  (params (`New Cargo` :type "/Game/Blueprints/BP_Cargo Object Reference"))
  (returns (isValid :type Boolean))
  (locals (isFull :type Boolean :default true) (TransformSpot :type "Transform Structure"))
  (for (_array_element _array_index) (`self.InventoryList`)
    (if (`/Game/Blueprints/BP_Cargo.isEmpty` _array_element)
      (`KismetArrayLibrary.Array_Add` (`self.EmptyCargoCache`) _array_element)
      (set `local.TransformSpot` (`Actor.GetTransform` _array_element))
      (`KismetArrayLibrary.Array_Set` (`self.InventoryList`) _array_index (`local.New Cargo`))
      (set `local.isFull` false)
      (`Actor.K2_SetActorTransform` (`local.New Cargo`) (`local.TransformSpot`) false false)
      (bind _asbp_quarter_base (cast `/Game/Blueprints/BP_QuarterBase` (`self.GetOwner`)))
      (`Actor.K2_AttachToComponent` (`local.New Cargo`) (`/Game/Blueprints/BP_QuarterBase.Shelf` _asbp_quarter_base) "None" "KeepWorld" "KeepWorld" "KeepWorld" true)
      (break)))
  (if (`local.isFull`)
    (return false)
    (else
      (return true))))

(fn `RemoveCargo`
  (params (CargoReference :type "/Game/Blueprints/BP_Cargo Object Reference"))
  (locals (Transform :type "Transform Structure"))
  (bind _output (`|GetArrayItem` (`self.EmptyCargoCache`)))
  (`/Game/Blueprints/BP_Cargo.DisableSelf` CargoReference)
  (set `local.Transform` (`Actor.GetTransform` CargoReference))
  (`KismetArrayLibrary.Array_Set` (`self.InventoryList`) (`KismetArrayLibrary.Array_Find` (`self.InventoryList`) CargoReference) _output)
  (`Actor.K2_SetActorTransform` _output (`local.Transform`) false false)
  (`KismetArrayLibrary.Array_Remove` (`self.EmptyCargoCache`)))