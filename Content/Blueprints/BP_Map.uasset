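; BP_Map is an interactive map actor where hovering and clicking stations selects a destination.
; On BeginPlay it finds the BP_QuarterBase and spawns an attached BP_Pin.
; Hovering moves a highlight effect beside the station and shows it, with no hide logic on hover end.
; Clicking moves the pin to the station and passes the station's object name to QuarterBase's ACMapSystem as the destination, with a debug print.
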(event `self.ReceiveBeginPlay`
  (bind _returnvalue (`GameplayStatics.GetActorOfClass` "/Game/Blueprints/BP_QuarterBase.BP_QuarterBase_C"))
  (set `self.QuarterBase` _returnvalue)
  (bind _returnvalue_2 (`|SpawnActorFromClass` "/Game/Blueprints/BP_Pin.BP_Pin_C" (`SceneComponent.K2_GetComponentToWorld` (`self.DefaultSceneRoot`)) "Undefined" "MultiplyWithRoot" null null))
  (bind _output_get (set `self.Pin` _returnvalue_2))
  (`self.K2_AttachToActor` _output_get self "None" "KeepWorld" "KeepWorld" "KeepWorld" true))

(event `MouseOverStation`
  (params (Station :type "PrimitiveComponent Object Reference"))
  (if (not (`SceneComponent.bVisible` (`self.HoverEffect`)))
    (`SceneComponent.SetVisibility` (`self.HoverEffect`) true false))
  (`SceneComponent.K2_SetRelativeLocation` (`self.HoverEffect`) (+ (`SceneComponent.RelativeLocation` Station) (3.0 -5.0 0.0)) false false))

(event `MouseFinishOver`
  (params (Station :type "PrimitiveComponent Object Reference")))

(event `MouseClickStation`
  (params (Station :type "PrimitiveComponent Object Reference"))
  (bind _returnvalue (`KismetSystemLibrary.GetObjectName` Station))
  (`|ExecutionSequence`
    (:`then_0`
      (`SceneComponent.K2_SetRelativeLocation` (`Actor.RootComponent` (`self.Pin`)) (`SceneComponent.RelativeLocation` Station) true false))
    (:`then_1`
      (`/Game/Blueprints/AC_MapSystem.SetDestination` (`/Game/Blueprints/BP_QuarterBase.AC_MapSystem` (`self.QuarterBase`)) (`KismetStringLibrary.Conv_StringToName` _returnvalue))
      (`KismetSystemLibrary.PrintString` (`KismetStringLibrary.Concat_StrStr` _returnvalue " is set to destination") true true (struct :`G` 0.104754 :`B` 1.0 :`A` 1.0) 200.0 "Destination"))))

(fn `UserConstructionScript`)