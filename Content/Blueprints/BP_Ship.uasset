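; BP_Ship is a ship that travels along its current line's spline at a set speed, forward or reversed.
; Each tick it updates position and yaw from spline distance, wrapping on closed loops and stopping at open ends.
; Debug keys toggle stopping and direction; BeginPlay places it at a station's landing point for take-off testing.
; TakeOff, currently not wired in, follows a station-built track to an attach point on the line.
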(event `Key|Up`
  (params (Key :type "Key Structure"))
  ;[1 1 1] Reverse On Track
  (:`Pressed`
    (`/Engine/EditorBlueprintResources/StandardMacros.FlipFlop`
      (:`A`
        (set `self.IsForwardOnLine` false))
      (:`B`
        (set `self.IsForwardOnLine` true)))))

(event `Key|Equals`
  (params (Key :type "Key Structure"))
  ;[1 1 1] Stop Logic
  (:`Pressed`
    (`/Engine/EditorBlueprintResources/StandardMacros.FlipFlop`
      (:`A`
        (set `self.StopFollow` true))
      (:`B`
        (set `self.StopFollow` false)))))

(event `self.ReceiveBeginPlay`
  (bind _returnvalue (`GameplayStatics.GetActorOfClass` "/Game/Blueprints/BP_NaviSystem.BP_NaviSystem_C"))
  (set `self.NaviSystem` _returnvalue)
  (set `self.CurrentSpline` (`/Game/Blueprints/BP_Spline_Road.Spline` (`self.CurrentLine`)))
  (set `self.InitialWorldRotation` (`SceneComponent.K2_GetComponentRotation` (`self.Ship`)))
  ;[1 1 1] Set to Station Landing World Location for Take Off Test
  (`SceneComponent.K2_SetWorldLocation` (`self.Ship`) (`/Game/Blueprints/BP_Station.WorldLocationLanding` (`self.AtStation`)) false false))

(event `self.ReceiveTick`
  (params (DeltaSeconds :type "Float (single-precision)"))
  (if (not (`self.StopFollow`))
    (`self.MoveAlongSpline` (`/Game/Blueprints/BP_Spline_Road.Spline` (`self.CurrentLine`)))))

(fn `MoveAlongSpline`
  (params (SplineToFollow :type "SplineComponent Object Reference"))
  (bind _splinetofollow (`local.SplineToFollow`))
  (bind _distancealongspline (`self.DistanceAlongSpline`))
  (bind _ship (`self.Ship`))
  (bind (_initialworldrotation_roll _initialworldrotation_pitch _initialworldrotation_yaw) (`KismetMathLibrary.BreakRotator` (`self.InitialWorldRotation`)))
  (bind _distancealongspline_2 (`self.DistanceAlongSpline`))
  (bind _splinetofollow_2 (`local.SplineToFollow`))
  (bind _returnvalue (`SplineComponent.GetSplineLength` _splinetofollow_2))
  (bind (_returnvalue_roll _returnvalue_pitch _returnvalue_yaw) (`KismetMathLibrary.BreakRotator` (`SplineComponent.GetRotationAtDistanceAlongSpline` _splinetofollow _distancealongspline "World")))
  (set `self.DistanceAlongSpline` (+ (* (* (`GameplayStatics.GetWorldDeltaSeconds`) (`self.Speed`)) (`self.FwdBwd`)) (`self.DistanceAlongSpline`)))
  (`SceneComponent.K2_SetWorldLocation` _ship (`SplineComponent.GetLocationAtDistanceAlongSpline` _splinetofollow _distancealongspline "World") false false)
  (`SceneComponent.K2_SetWorldRotation` _ship (`KismetMathLibrary.MakeRotator` _initialworldrotation_roll _initialworldrotation_pitch (+ (+ _initialworldrotation_yaw _returnvalue_yaw) (* (- 1.0 (`KismetMathLibrary.Conv_BoolToDouble` (`self.IsForwardOnLine`))) 180.0))) false false)
  (if (`SplineComponent.IsClosedLoop` _splinetofollow_2)
    (set `self.DistanceAlongSpline` (mod (`self.DistanceAlongSpline`) _returnvalue))
    (elif (or (>= _distancealongspline_2 _returnvalue) (<= _distancealongspline_2 0.0))
      (set `self.DistanceAlongSpline` (`KismetMathLibrary.FClamp` (`self.DistanceAlongSpline`) 0.0 _returnvalue))
      (set `self.StopFollow` true))))

(fn `TakeOff`
  (locals (HasSetup :type Boolean) (AttachPointInputKey :type "Float (double-precision)"))
  (bind _atstation (`self.AtStation`))
  (if (not (`local.HasSetup`))
    (bind _output_get (set `local.AttachPointInputKey` (+ (`BlueprintMapLibrary.Map_Find` (`/Game/Blueprints/BP_Station.InputKeysOnLines` (`self.AtStation`)) (`self.CurrentLineIndex`)) (* (`self.FwdBwd`) 0.5))))
    (`/Game/Blueprints/BP_Station.SetTakeOffTrack` _atstation (`SplineComponent.GetLocationAtSplineInputKey` (`/Game/Blueprints/BP_Spline_Road.Spline` (`self.CurrentLine`)) _output_get "World"))
    (bind _output_get_2 (set `self.CurrentSpline` (`/Game/Blueprints/BP_Station.TakeOffTrack` _atstation)))
    (set `local.HasSetup` true))
  (`self.MoveAlongSpline` _output_get_2)
  (if (`self.StopFollow`)
    (`|ExecutionSequence`
      (:`then_0`
        (set `self.CurrentSpline` (`/Game/Blueprints/BP_Spline_Road.Spline` (`self.CurrentLine`))))
      (:`then_1`
        (set `self.DistanceAlongSpline` (`SplineComponent.GetDistanceAlongSplineAtSplineInputKey` (`self.CurrentSpline`) (`local.AttachPointInputKey`)))))))

(fn `UserConstructionScript`)