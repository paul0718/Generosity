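; AC_DebugTool is a debug component on BP_QuarterBase that binds keyboard keys to shortcuts for testing game systems.
; BeginPlay caches the owning QuarterBase, and key events call into its flow control, quest, inventory, map and steering components.
; Shortcuts switch flow states, land, end the game, toggle doors, add or remove cargo, manage quests and unlock map lines, with FlipFlops alternating paired actions.
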(event `Key|Two`
  (params (Key :type "Key Structure"))
  (:`Pressed`
    (`/Engine/EditorBlueprintResources/StandardMacros.FlipFlop`
      (:`A`
        (`/Game/Blueprints/AC_FlowControl.SwitchToState` (`/Game/Blueprints/BP_QuarterBase.AC_FlowControl` (`self.QuarterBase`)) "NewEnumerator0"))
      (:`B`
        (`/Game/Blueprints/AC_FlowControl.SwitchToState` (`/Game/Blueprints/BP_QuarterBase.AC_FlowControl` (`self.QuarterBase`)) "NewEnumerator1")))))

(event `Key|NumPadOne`
  (params (Key :type "Key Structure"))
  (:`Pressed`
    (`self.UnlockNextLine`)))

(event `Key|Enter`
  (params (Key :type "Key Structure"))
  (:`Pressed`
    (`/Game/Blueprints/AC_FlowControl.Game End` (`/Game/Blueprints/BP_QuarterBase.AC_FlowControl` (`self.QuarterBase`)))))

(event `Key|Zero`
  (params (Key :type "Key Structure"))
  (bind _quarterbase (`self.QuarterBase`))
  (:`Pressed`
    (`/Engine/EditorBlueprintResources/StandardMacros.FlipFlop`
      (:`A`
        (`/Game/Blueprints/BP_QuarterBase.OpenDoor` _quarterbase))
      (:`B`
        (`/Game/Blueprints/BP_QuarterBase.CloseDoor` _quarterbase)))))

(event `Key|NumPadFour`
  (params (Key :type "Key Structure"))
  (bind _ac_questmanager (`/Game/Blueprints/BP_QuarterBase.AC_QuestManager` (`self.QuarterBase`)))
  (:`Pressed`
    (`/Game/Blueprints/AC_QuestManager.Add Quest to Log` _ac_questmanager (`/Game/Blueprints/AC_QuestManager.ConstructedQuest` _ac_questmanager))))

(event `Key|C`
  (params (Key :type "Key Structure"))
  (:`Pressed`
    (`self.Remove The First Cargo`)))

(event `Key|Backslash`
  (params (Key :type "Key Structure"))
  (:`Pressed`
    (`/Game/Blueprints/AC_FlowControl.Lands` (`/Game/Blueprints/BP_QuarterBase.AC_FlowControl` (`self.QuarterBase`)))))

(event `Key|NumPadFive`
  (params (Key :type "Key Structure"))
  (:`Pressed`
    (`self.AddQuest`)))

(event `Key|X`
  (params (Key :type "Key Structure"))
  (:`Pressed`
    (`/Engine/EditorBlueprintResources/StandardMacros.FlipFlop`
      (:`A`
        (`self.AddNewCargoOfClass` "/Game/Blueprints/CargoLibrary/BI_Cargo_Aloe.BI_Cargo_Aloe_C"))
      (:`B`
        (`self.AddNewCargoOfClass` "/Game/Blueprints/CargoLibrary/BI_Cargo_Crystal.BI_Cargo_Crystal_C")))))

(event `Key|NumPadSix`
  (params (Key :type "Key Structure"))
  (:`Pressed`
    (`self.PassRound`)))

(event `Key|NumPadSeven`
  (params (Key :type "Key Structure"))
  (:`Pressed`
    (`self.DeleteQuest`)))

(event `Key|Z`
  (params (Key :type "Key Structure"))
  (:`Pressed`
    (`/Game/Blueprints/AC_SteerSystem.TurnAround` (`/Game/Blueprints/BP_QuarterBase.AC_SteerSystem` (`self.QuarterBase`)))))

(event `self.ReceiveBeginPlay`
  (bind _asbp_quarter_base (cast `/Game/Blueprints/BP_QuarterBase` (`self.GetOwner`)))
  (set `self.QuarterBase` _asbp_quarter_base))

(fn `AddNewCargoOfClass`
  (params (`Cargo BI` :type "/Game/Blueprints/BP_Cargo Class Reference"))
  (bind _asbp_quarter_base (cast `/Game/Blueprints/BP_QuarterBase` (`self.GetOwner`)))
  (`/Game/Blueprints/AC_Inventory.AddCargoOfClass` (`/Game/Blueprints/BP_QuarterBase.AC_Inventory` _asbp_quarter_base) `Cargo BI`))

(fn `AddQuest`
  (`/Game/Blueprints/AC_QuestManager.Draw Quest At Station` (`/Game/Blueprints/BP_QuarterBase.AC_QuestManager` (`self.QuarterBase`))))

(fn `DeleteQuest`
  (bind _ac_questmanager (`/Game/Blueprints/BP_QuarterBase.AC_QuestManager` (`self.QuarterBase`)))
  (bind _output (`|GetArrayItem` (`/Game/Blueprints/AC_QuestManager.QuestList` _ac_questmanager)))
  (`/Engine/EditorBlueprintResources/StandardMacros.IsValid` _output
    (:`Is Valid`
      (`/Game/Blueprints/AC_QuestManager.Remove Quest` _ac_questmanager _output))
    (:`Is Not Valid`
      (`KismetSystemLibrary.PrintString` "Quest Log is Null" true true (struct :`R` 1.0 :`G` 0.923259 :`B` 0.155993 :`A` 1.0)))))

(fn `MoveBoatUpByX`
  (params (Distance :type "Float (double-precision)"))
  (bind _returnvalue (`self.GetOwner`))
  (bind (_returnvalue_location _returnvalue_rotation _returnvalue_scale) (`KismetMathLibrary.BreakTransform` (`Actor.GetTransform` _returnvalue)))
  (`Actor.K2_SetActorTransform` _returnvalue (`KismetMathLibrary.MakeTransform` (+ _returnvalue_location (`KismetMathLibrary.MakeVector` 0.0 0.0 Distance)) _returnvalue_rotation _returnvalue_scale) false false))

(fn `PassRound`
  (`/Game/Blueprints/AC_QuestManager.Pass Round for Quests` (`/Game/Blueprints/BP_QuarterBase.AC_QuestManager` (`self.QuarterBase`))))

(fn `Remove The First Cargo`
  (for _array_element (`/Game/Blueprints/AC_Inventory.InventoryList` (`/Game/Blueprints/BP_QuarterBase.AC_Inventory` (`self.QuarterBase`)))
    (if (not (`/Game/Blueprints/BP_Cargo.isEmpty` _array_element))
      (`/Game/Blueprints/AC_Inventory.RemoveCargo` (`/Game/Blueprints/BP_QuarterBase.AC_Inventory` (`self.QuarterBase`)) _array_element)
      (break))))

(fn `ToggleRoamMovement`)

(fn `UnlockNextLine`
  (`/Game/Blueprints/AC_MapSystem.Unlock Line` (`/Game/Blueprints/BP_QuarterBase.AC_MapSystem` (`self.QuarterBase`)) 1 (`self.mapindex`))
  (`/Engine/EditorBlueprintResources/StandardMacros.IncrementInt` (`self.mapindex`)))