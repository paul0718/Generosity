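; Quest actor for delivery and escort quests, showing goal, destination, round progress and status through decals, text and marks.
; ConstructQuest builds visuals by tier and type, randomizing tier-1 cargo.
; CheckQuestStatus tests round expiry, then inventory or ship station; category quests briefly spawn each item to read its Type.
; PassRound reveals round marks, while check/X clicks call BP_QuarterBase's quest manager, also notifying flow control at the Gate.
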(event `self.ReceiveBeginPlay`
  (`|ExecutionSequence`
    (:`then_0`
      (`PrimitiveComponent.SetCollisionEnabled` (`self.XMarkCollision`) "NoCollision")
      (`PrimitiveComponent.SetCollisionEnabled` (`self.CheckMarkCollision`) "NoCollision"))
    (:`then_1`
      (bind _keys (`BlueprintMapLibrary.Map_Keys` (`self.Items and Number`)))
      (for _array_element _keys
        (`BlueprintMapLibrary.Map_Add` (`self.OnHand Items and Number`) _array_element)))
    (:`then_2`
      (bind _returnvalue (`GameplayStatics.GetActorOfClass` "/Game/Blueprints/BP_QuarterBase.BP_QuarterBase_C"))
      (set `self.QuarterBase` _returnvalue))))

(event `Hover Check Mark`
  (params (`Which Mark` :type "PrimitiveComponent Object Reference")))

(event `End Hover Check Mark`
  (params (`Which Mark` :type "PrimitiveComponent Object Reference")))

(event `Click Check Mark`
  (params (WhichMark :type "PrimitiveComponent Object Reference") (`Under Location` :type "/Game/Blueprints/EM_InteractLocations Enum" :default "NewEnumerator8"))
  (switch `/Game/Blueprints/EM_InteractLocations` `Under Location`
    (:`NewEnumerator1`
      (switch `string` (`KismetSystemLibrary.GetObjectName` (`SceneComponent.GetChildComponent` WhichMark 0))
        (:`CheckMark`
          (`/Game/Blueprints/AC_QuestManager.Complete Quest` (`/Game/Blueprints/BP_QuarterBase.AC_QuestManager` (`self.QuarterBase`)) self))
        (:`XMark`
          (`/Game/Blueprints/AC_QuestManager.Remove Quest` (`/Game/Blueprints/BP_QuarterBase.AC_QuestManager` (`self.QuarterBase`)) self))))
    (:`NewEnumerator2`
      (switch `string` (`KismetSystemLibrary.GetObjectName` (`SceneComponent.GetChildComponent` WhichMark 0))
        (:`CheckMark`
          (`/Game/Blueprints/AC_QuestManager.Add Quest to Log` (`/Game/Blueprints/BP_QuarterBase.AC_QuestManager` (`self.QuarterBase`)) self))
        (:`XMark`
          (`/Game/Blueprints/AC_QuestManager.Remove Quest` (`/Game/Blueprints/BP_QuarterBase.AC_QuestManager` (`self.QuarterBase`)) self)))
      (`/Game/Blueprints/AC_FlowControl.Picked up/Gave up Quest` (`/Game/Blueprints/BP_QuarterBase.AC_FlowControl` (`self.QuarterBase`)) (not (`KismetMathLibrary.Conv_IntToBool` (`self.Tier`)))))))

(fn `Check Quest Status`
  (params (InventoryMap :type "Map of /Game/Blueprints/BP_Cargo Class Reference to Integer"))
  (returns (StatusText :type "/Game/Blueprints/EM_QuestStatus Enum"))
  (locals (isRequirementFulfilled :type Boolean :default true) (NumberCount :type Integer))
  (switch `/Game/Blueprints/EM_QuestType` (`self.QuestType`)
    (:`NewEnumerator0`
      (`|ExecutionSequence`
        (:`then_0`
          (set `self.OnHand Items and Number` (`local.InventoryMap`)))
        (:`then_1`
          (if (`self.ItemClassOverSpecie`)
            (if (> (`self.CurrentRound`) (`self.RoundLimit`))
              (bind _output_get (set `self.Status` "NewEnumerator2"))
              (`SceneComponent.SetVisibility` (`self.ExpiredMark`) true false)
              (return _output_get)
              (else
                (bind _keys (`BlueprintMapLibrary.Map_Keys` (`self.OnHand Items and Number`)))
                (set `local.NumberCount` 0)
                (for _array_element _keys
                  (bind _returnvalue (`|SpawnActorFromClass` _array_element (`KismetMathLibrary.MakeTransform` (0.0 0.0 0.0)) "Undefined" "MultiplyWithRoot" null null))
                  (if (`|EnumEquality` (`/Game/Blueprints/BP_Cargo.Type` _returnvalue) (`self.ItemClasses and 4 for Tier 0`))
                    (set `local.NumberCount` (+ (`BlueprintMapLibrary.Map_Find` (`self.OnHand Items and Number`) _array_element) (`local.NumberCount`))))
                  (`self.K2_DestroyActor` _returnvalue))
                (if (>= (`local.NumberCount`) 4)
                  (set `self.Status` "NewEnumerator1")
                  (`self.Show Fulfill Mark` true)
                  (else
                    (set `self.Status` "NewEnumerator0")
                    (`self.Show Fulfill Mark` false)))
                (return (`self.Status`))))
            (else
              ;[1 1 1] Status Check
              (if (> (`self.CurrentRound`) (`self.RoundLimit`))
                (bind _output_get_2 (set `self.Status` "NewEnumerator2"))
                (`SceneComponent.SetVisibility` (`self.ExpiredMark`) true false)
                (return _output_get_2)
                (else
                  (bind _keys_2 (`BlueprintMapLibrary.Map_Keys` (`self.Items and Number`)))
                  (for _array_element_2 _keys_2
                    (bind (_value _returnvalue_2) (`BlueprintMapLibrary.Map_Find` (`self.OnHand Items and Number`) _array_element_2))
                    (if (not (and (>= _value (`BlueprintMapLibrary.Map_Find` (`self.Items and Number`) _array_element_2)) _returnvalue_2))
                      (set `local.isRequirementFulfilled` false)))
                  (if (`local.isRequirementFulfilled`)
                    (set `self.Status` "NewEnumerator1")
                    (`self.Show Fulfill Mark` true)
                    (else
                      (set `self.Status` "NewEnumerator0")
                      (`self.Show Fulfill Mark` false)))
                  (return (`self.Status`)))))))))
    (:`NewEnumerator2`
      (if (> (`self.CurrentRound`) (`self.RoundLimit`))
        (bind _output_get_3 (set `self.Status` "NewEnumerator2"))
        (`SceneComponent.SetVisibility` (`self.ExpiredMark`) true false)
        (return _output_get_3)
        (else
          (if (== (`/Game/Blueprints/ShipMovement/AC_ShipController.AtStation` (`/Game/Blueprints/BP_QuarterBase.AC_ShipController` (`self.QuarterBase`))) (`self.Destination Station`))
            (set `self.Status` "NewEnumerator1")
            (`self.Show Fulfill Mark` true)
            (else
              (set `self.Status` "NewEnumerator0")
              (`self.Show Fulfill Mark` false)))
          (return (`self.Status`)))))))

(fn `ConstructQuest`
  (params (DestinationStation :type "/Game/Blueprints/BP_Station Object Reference"))
  (bind _towntextdelivery (`self.TownTextDelivery`))
  (bind _questt1_location (`self.QuestT1_Location`))
  (bind _towntextdelivery_2 (`self.TownTextDelivery`))
  (bind _questt1_location_2 (`self.QuestT1_Location`))
  (switch `int` (`self.Tier`)
    (:`1`
      (switch `/Game/Blueprints/EM_QuestType` (`self.QuestType`)
        (:`NewEnumerator0`
          ;[1 1 1 1 89] Construct Delivery Quest T1
          (`SceneComponent.SetVisibility` (`self.QuestTypeDelivery`) true false)
          (`SceneComponent.SetVisibility` (`self.QuestT1_DeliveryBase`) true false)
          (bind _output_get (set `self.Tier1ResourceType` (cast `/Game/Blueprints/EM_ResourceType` (`KismetMathLibrary.Conv_IntToByte` (`KismetMathLibrary.RandomInteger` (`self.ResourceListSize`))))))
          (switch `/Game/Blueprints/EM_ResourceType` _output_get
            (:`NewEnumerator0`
              (`SceneComponent.SetVisibility` (`self.QuestT1_Beef`) true false)
              (`BlueprintMapLibrary.Map_Add` (`self.Items and Number`) "/Game/Blueprints/CargoLibrary/BI_Cargo_Beef.BI_Cargo_Beef_C" 1)
              (`TextRenderComponent.K2_SetText` (`self.TownTextDelivery`) (`KismetTextLibrary.Conv_NameToText` (`/Game/Blueprints/BP_Station.Name` (`local.DestinationStation`))) :!label _label)
              (`DecalComponent.SetDecalMaterial` (`self.QuestT1_Location`) (`/Game/Blueprints/BP_Station.Sprite` (`local.DestinationStation`)))
              (`SceneComponent.SetVisibility` (`self.QuestT1_Location`) true false)
              (set `self.Destination Station` (`local.DestinationStation`)))
            (:`NewEnumerator1`
              (`SceneComponent.SetVisibility` (`self.QuestT1_Chicken`) true false)
              (`BlueprintMapLibrary.Map_Add` (`self.Items and Number`) "/Game/Blueprints/CargoLibrary/BI_Cargo_Chicken.BI_Cargo_Chicken_C" 1)
              (goto _label))
            (:`NewEnumerator2`
              (`SceneComponent.SetVisibility` (`self.QuestT1_Shrimp`) true false)
              (`BlueprintMapLibrary.Map_Add` (`self.Items and Number`) "/Game/Blueprints/CargoLibrary/BI_Cargo_Shrimp.BI_Cargo_Shrimp_C" 1)
              (goto _label))
            (:`NewEnumerator3`
              (`SceneComponent.SetVisibility` (`self.QuestT1_Fish`) true false)
              (`BlueprintMapLibrary.Map_Add` (`self.Items and Number`) "/Game/Blueprints/CargoLibrary/BI_Cargo_Fish.BI_Cargo_Fish_C" 1)
              (goto _label))
            (:`NewEnumerator4`
              (`SceneComponent.SetVisibility` (`self.QuestT1_Rose`) true false)
              (`BlueprintMapLibrary.Map_Add` (`self.Items and Number`) "/Game/Blueprints/CargoLibrary/BI_Cargo_Rose.BI_Cargo_Rose_C" 1)
              (goto _label))
            (:`NewEnumerator5`
              (`SceneComponent.SetVisibility` (`self.QuestT1_Lily`) true false)
              (`BlueprintMapLibrary.Map_Add` (`self.Items and Number`) "/Game/Blueprints/CargoLibrary/BI_Cargo_Lily.BI_Cargo_Lily_C" 1)
              (goto _label))
            (:`NewEnumerator6`
              (`SceneComponent.SetVisibility` (`self.QuestT1_Cactus`) true false)
              (`BlueprintMapLibrary.Map_Add` (`self.Items and Number`) "/Game/Blueprints/CargoLibrary/BI_Cargo_Cactus.BI_Cargo_Cactus_C" 1)
              (goto _label))
            (:`NewEnumerator7`
              (`SceneComponent.SetVisibility` (`self.QuestT1_Aloe`) true false)
              (`BlueprintMapLibrary.Map_Add` (`self.Items and Number`) "/Game/Blueprints/CargoLibrary/BI_Cargo_Aloe.BI_Cargo_Aloe_C" 1)
              (goto _label))
            (:`NewEnumerator8`
              (`SceneComponent.SetVisibility` (`self.QuestT1_Gold`) true false)
              (`BlueprintMapLibrary.Map_Add` (`self.Items and Number`) "/Game/Blueprints/CargoLibrary/BI_Cargo_Gold.BI_Cargo_Gold_C" 1)
              (goto _label))
            (:`NewEnumerator9`
              (`SceneComponent.SetVisibility` (`self.QuestT1_Bronze`) true false)
              (`BlueprintMapLibrary.Map_Add` (`self.Items and Number`) "/Game/Blueprints/CargoLibrary/BI_Cargo_Bronze.BI_Cargo_Bronze_C" 1)
              (goto _label))
            (:`NewEnumerator10`
              (`SceneComponent.SetVisibility` (`self.QuestT1_Pearl`) true false)
              (`BlueprintMapLibrary.Map_Add` (`self.Items and Number`) "/Game/Blueprints/CargoLibrary/BI_Cargo_Pearl.BI_Cargo_Pearl_C" 1)
              (goto _label))
            (:`NewEnumerator11`
              (`SceneComponent.SetVisibility` (`self.QuestT1_Coral`) true false)
              (`BlueprintMapLibrary.Map_Add` (`self.Items and Number`) "/Game/Blueprints/CargoLibrary/BI_Cargo_Coral.BI_Cargo_Coral_C" 1)
              (goto _label))
            (:`NewEnumerator12`
              (`SceneComponent.SetVisibility` (`self.QuestT1_Iron`) true false)
              (`BlueprintMapLibrary.Map_Add` (`self.Items and Number`) "/Game/Blueprints/CargoLibrary/BI_Cargo_Iron.BI_Cargo_Iron_C" 1)
              (goto _label))
            (:`NewEnumerator13`
              (`SceneComponent.SetVisibility` (`self.QuestT1_Obsidian`) true false)
              (`BlueprintMapLibrary.Map_Add` (`self.Items and Number`) "/Game/Blueprints/CargoLibrary/BI_Cargo_Obsidian.BI_Cargo_Obsidian_C" 1)
              (goto _label))
            (:`NewEnumerator14`
              (`SceneComponent.SetVisibility` (`self.QuestT1_Diamond`) true false)
              (`BlueprintMapLibrary.Map_Add` (`self.Items and Number`) "/Game/Blueprints/CargoLibrary/BI_Cargo_Diamond.BI_Cargo_Diamond_C" 1)
              (goto _label))
            (:`NewEnumerator15`
              (`SceneComponent.SetVisibility` (`self.QuestT1_Crystal`) true false)
              (`BlueprintMapLibrary.Map_Add` (`self.Items and Number`) "/Game/Blueprints/CargoLibrary/BI_Cargo_Crystal.BI_Cargo_Crystal_C" 1))))
        (:`NewEnumerator1`
          ;[1 1 1] Reach a destination State Machine
          (`|ExecutionSequence` :!label _label_2
            (:`then_0`
              (`SceneComponent.SetVisibility` (`self.QuestTypeEscort`) true false)
              (`SceneComponent.SetVisibility` (`self.QuestT1_EscortBase`) true false)
              (`TextRenderComponent.K2_SetText` (`self.TownTextDelivery`) (`KismetTextLibrary.Conv_NameToText` (`/Game/Blueprints/BP_Station.Name` (`local.DestinationStation`))))
              (`DecalComponent.SetDecalMaterial` (`self.QuestT1_Location`) (`/Game/Blueprints/BP_Station.Sprite` (`local.DestinationStation`)))
              (`SceneComponent.SetVisibility` (`self.QuestT1_Location`) true false)
              (set `self.Destination Station` (`local.DestinationStation`)))
            (:`then_1`
              (`SceneComponent.K2_SetRelativeLocation` _towntextdelivery_2 (+ (`SceneComponent.RelativeLocation` _towntextdelivery_2) (-10.0 0.0 0.0)) false false)
              (`SceneComponent.K2_SetRelativeLocation` _questt1_location_2 (+ (`SceneComponent.RelativeLocation` _questt1_location_2) (-10.0 0.0 0.0)) false false))))
        (:`NewEnumerator2`
          (goto _label_2))))
    (:`2`
      ;[1 1 1] Tier 2
      (switch `/Game/Blueprints/EM_QuestType` (`self.QuestType`)
        (:`NewEnumerator2`
          (`|ExecutionSequence`
            (:`then_0`
              (`SceneComponent.SetVisibility` (`self.QuestTypeEscort`) true false)
              (`SceneComponent.SetVisibility` (`self.QuestT1_EscortBase`) true false)
              (`TextRenderComponent.K2_SetText` (`self.TownTextDelivery`) (`KismetTextLibrary.Conv_NameToText` (`/Game/Blueprints/BP_Station.Name` (`local.DestinationStation`))))
              (`DecalComponent.SetDecalMaterial` (`self.QuestT1_Location`) (`/Game/Blueprints/BP_Station.Sprite` (`local.DestinationStation`)))
              (`SceneComponent.SetVisibility` (`self.QuestT1_Location`) true false)
              (set `self.Destination Station` (`local.DestinationStation`)))
            (:`then_1`
              (`SceneComponent.K2_SetRelativeLocation` _towntextdelivery (+ (`SceneComponent.RelativeLocation` _towntextdelivery) (-10.0 0.0 0.0)) false false)
              (`SceneComponent.K2_SetRelativeLocation` _questt1_location (+ (`SceneComponent.RelativeLocation` _questt1_location) (-10.0 0.0 0.0)) false false))))))))

(fn `PassRound`
  (`/Engine/EditorBlueprintResources/StandardMacros.IncrementInt` (`self.CurrentRound`)
    (:`  `
      (if (== (`self.RoundLimit`) 5)
        (switch `int` (`self.CurrentRound`)
          (:`1`
            (`SceneComponent.SetVisibility` (`self.PassMarks`) true false))
          (:`2`
            (`SceneComponent.SetVisibility` (`self.PassMarks1`) true false))
          (:`3`
            (`SceneComponent.SetVisibility` (`self.PassMarks2`) true false))
          (:`4`
            (`SceneComponent.SetVisibility` (`self.PassMarks3`) true false))
          (:`5`
            (`SceneComponent.SetVisibility` (`self.PassMarks4`) true false)))
        (elif (== (`self.RoundLimit`) 25)
          (switch `int` (/ (`self.CurrentRound`) 5)
            (:`1`
              (`SceneComponent.SetVisibility` (`self.PassMarks`) true false))
            (:`2`
              (`SceneComponent.SetVisibility` (`self.PassMarks1`) true false))
            (:`3`
              (`SceneComponent.SetVisibility` (`self.PassMarks2`) true false))
            (:`4`
              (`SceneComponent.SetVisibility` (`self.PassMarks3`) true false))
            (:`5`
              (`SceneComponent.SetVisibility` (`self.PassMarks4`) true false))))))))

(fn `Show Fulfill Mark`
  (params (On :type Boolean))
  (`SceneComponent.SetVisibility` (`self.FulfillMark`) On false))

(fn `UserConstructionScript`)