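; Actor component on BP_QuarterBase that drives the ship's game loop of landing, quest turn-in and pickup, takeoff, and game end.
; BeginPlay shows a loading screen, then lands at a station and opens a paused tutorial.
; Flow events call the quest, ship, compass and map components and change phase through SwitchToState.
; Each phase toggles trigger collision and prompt widgets, and most also show an info popup.
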(event `self.ReceiveBeginPlay`
  (bind _asbp_quarter_base (cast `/Game/Blueprints/BP_QuarterBase` (`self.GetOwner`)))
  (set `self.Quarter Base` _asbp_quarter_base)
  (bind _returnvalue (`|CreateWidget` "/Game/Blueprints/W_LoadingScreen.W_LoadingScreen_C" (`GameplayStatics.GetPlayerController` 0)))
  (`UserWidget.AddToViewport` _returnvalue 0)
  (`KismetSystemLibrary.Delay` 3.0)
  (`self.Start Game`)
  (`Widget.RemoveFromParent` _returnvalue))

(event `Start Game`
  (`|ExecutionSequence`
    (:`then_0`
      (`self.Lands`))
    (:`then_1`
      ;[1 1 1] Tutorial
      (`self.DrawTutorial`))))

(event `Picked up/Gave up Quest`
  (params (`At Main Stops` :type Boolean))
  (if `At Main Stops`
    (set `self.Tier0FinishedPickUp` true)
    (`self.T0_Setoff`)
    (else
      (`|ExecutionSequence` :!label _label
        (:`then_0`
          (`/Game/Blueprints/BP_QuarterBase.CloseDoor` (`self.Quarter Base`)))
        (:`then_1`
          (`self.SwitchToState` "NewEnumerator0"))
        (:`then_2`
          (`/Game/FirstPerson/Blueprints/BP_FirstPersonCharacter.Forced IA_Back` (`/Game/Blueprints/BP_QuarterBase.FirstPersonCharacter` (`self.Quarter Base`))))))))

(event `Gained Resources`
  (goto _label))

(event `Finish Turning in quests`
  (params (`At Main Stops` :type Boolean))
  (if `At Main Stops`
    (set `self.Tier0FinishedTurnin` true)
    (`self.T0_Setoff`)
    (else
      (`|ExecutionSequence` :!label _label_2
        (:`then_0`
          (`/Game/Blueprints/BP_QuarterBase.CloseDoor` (`self.Quarter Base`)))
        (:`then_1`
          (`self.SwitchToState` "NewEnumerator0"))
        (:`then_2`
          (`/Game/FirstPerson/Blueprints/BP_FirstPersonCharacter.Forced IA_Back` (`/Game/Blueprints/BP_QuarterBase.FirstPersonCharacter` (`self.Quarter Base`))))
        (:`then_3`
          (set `self.Tier0FinishedTurnin` false)
          (set `self.Tier0FinishedPickUp` false))))))

(event `Takes off`
  (bind _quarter_base (`self.Quarter Base`))
  (`|ExecutionSequence`
    (:`then_0`
      (`self.SwitchToState` "NewEnumerator1"))
    (:`then_1`
      (`/Game/Blueprints/AC_QuestManager.Pass Round for Quests` (`/Game/Blueprints/BP_QuarterBase.AC_QuestManager` (`self.Quarter Base`))))
    (:`then_2`
      (set `/Game/Blueprints/ShipMovement/AC_ShipController.StepsLeft` (`/Game/Blueprints/AC_CompassSystem.Roll` (`/Game/Blueprints/BP_QuarterBase.AC_CompassSystem` _quarter_base)) (`/Game/Blueprints/BP_QuarterBase.AC_ShipController` _quarter_base)))
    (:`then_3`
      (`/Game/Blueprints/ShipMovement/AC_ShipController.Confirm and Set off` (`/Game/Blueprints/BP_QuarterBase.AC_ShipController` (`self.Quarter Base`))))))

(event `T0_Setoff`
  (if (and (`self.Tier0FinishedTurnin`) (`self.Tier0FinishedPickUp`))
    (goto _label_2)))

(event `Game End`
  (`GameplayStatics.OpenLevelBySoftObjectPtr` "/Game/Levels/EndMenu.EndMenu"))

(event `Lands`
  (`|ExecutionSequence`
    (:`then_0`
      (`self.SwitchToState` "NewEnumerator4"))
    (:`then_1`
      (`/Game/Blueprints/BP_QuarterBase.OpenDoor` (`self.Quarter Base`)))
    (:`then_2`
      (`/Game/Blueprints/AC_QuestManager.Update Quest Status` (`/Game/Blueprints/BP_QuarterBase.AC_QuestManager` (`self.Quarter Base`))))
    (:`then_3`
      (`/Game/Blueprints/AC_QuestManager.ExecuteActions` (`/Game/Blueprints/BP_QuarterBase.AC_QuestManager` (`self.Quarter Base`))))
    (:`then_4`
      (`/Game/Blueprints/AC_MapSystem.UpdateShipIconLocation` (`/Game/Blueprints/BP_QuarterBase.AC_MapSystem` (`self.Quarter Base`))))))

(event `EnterSteerMode`)

(fn `DrawTutorial`
  (bind _returnvalue (`|CreateWidget` "/Game/Blueprints/W_Tutorial.W_Tutorial_C" (`GameplayStatics.GetPlayerController` 0)))
  (`UserWidget.AddToViewport` _returnvalue 0)
  (`GameplayStatics.SetGamePaused` true)
  (set `PlayerController.bShowMouseCursor` true (`GameplayStatics.GetPlayerController` 0)))

(fn `PopupText`
  (bind _returnvalue (`WidgetComponent.GetWidget` (`/Game/Blueprints/BP_QuarterBase.Infotext` (`self.Quarter Base`))))
  (switch `/Game/Blueprints/EM_Phase` (`self.CurrentState`)
    (:`NewEnumerator0`
      (bind _asw_info_popup (cast `/Game/Blueprints/W_InfoPopup` _returnvalue))
      (`/Game/Blueprints/W_InfoPopup.Give Popup` _asw_info_popup "At Station"))
    (:`NewEnumerator3`
      (bind _asw_info_popup_2 (cast `/Game/Blueprints/W_InfoPopup` _returnvalue))
      (`/Game/Blueprints/W_InfoPopup.Give Popup` _asw_info_popup_2 "Steering Required"))
    (:`NewEnumerator4`
      (bind _asw_info_popup_3 (cast `/Game/Blueprints/W_InfoPopup` _returnvalue))
      (`/Game/Blueprints/W_InfoPopup.Give Popup` _asw_info_popup_3 "Interact With the Station!"))))

(fn `Restore To Current State Default`
  (`self.SwitchToState` (`self.CurrentState`)))

(fn `SwitchToState`
  (params (Phase :type "/Game/Blueprints/EM_Phase Enum" :default "NewEnumerator0"))
  (bind _quarter_base (`self.Quarter Base`))
  (bind _quarter_base_2 (`self.Quarter Base`))
  (bind _quarter_base_3 (`self.Quarter Base`))
  (bind _quarter_base_4 (`self.Quarter Base`))
  (bind _quarter_base_5 (`self.Quarter Base`))
  (bind _quarter_base_6 (`self.Quarter Base`))
  (bind _quarter_base_7 (`self.Quarter Base`))
  (bind _quarter_base_8 (`self.Quarter Base`))
  (bind _doortrigger (`/Game/Blueprints/BP_QuarterBase.DoorTrigger` _quarter_base))
  (bind _doortrigger_2 (`/Game/Blueprints/BP_QuarterBase.DoorTrigger` _quarter_base_2))
  (bind _npctrigger (`/Game/Blueprints/BP_QuarterBase.NPCTrigger` _quarter_base_2))
  (bind _questtrigger (`/Game/Blueprints/BP_QuarterBase.QuestTrigger` _quarter_base_2))
  (bind _tableinteracttrigger (`/Game/Blueprints/BP_QuarterBase.TableInteractTrigger` _quarter_base_2))
  (bind _steertrigger (`/Game/Blueprints/BP_QuarterBase.SteerTrigger` _quarter_base_2))
  (bind _doortrigger_3 (`/Game/Blueprints/BP_QuarterBase.DoorTrigger` _quarter_base_4))
  (bind _npctrigger_2 (`/Game/Blueprints/BP_QuarterBase.NPCTrigger` _quarter_base_4))
  (bind _doortrigger_4 (`/Game/Blueprints/BP_QuarterBase.DoorTrigger` _quarter_base_8))
  (bind _questtrigger_2 (`/Game/Blueprints/BP_QuarterBase.QuestTrigger` _quarter_base_4))
  (bind _tableinteracttrigger_2 (`/Game/Blueprints/BP_QuarterBase.TableInteractTrigger` _quarter_base_4))
  (bind _steertrigger_2 (`/Game/Blueprints/BP_QuarterBase.SteerTrigger` _quarter_base_4))
  (bind _scenerytrigger (`/Game/Blueprints/BP_QuarterBase.SceneryTrigger` _quarter_base_2))
  (bind _scenerytrigger_2 (`/Game/Blueprints/BP_QuarterBase.SceneryTrigger` _quarter_base_8))
  (bind _scenerytrigger_3 (`/Game/Blueprints/BP_QuarterBase.SceneryTrigger` _quarter_base_4))
  (bind _questtrigger_3 (`/Game/Blueprints/BP_QuarterBase.QuestTrigger` _quarter_base))
  (bind _tableinteracttrigger_3 (`/Game/Blueprints/BP_QuarterBase.TableInteractTrigger` _quarter_base))
  (bind _steertrigger_3 (`/Game/Blueprints/BP_QuarterBase.SteerTrigger` _quarter_base))
  (bind _npctrigger_3 (`/Game/Blueprints/BP_QuarterBase.NPCTrigger` _quarter_base_8))
  (bind _scenerytrigger_4 (`/Game/Blueprints/BP_QuarterBase.SceneryTrigger` _quarter_base))
  (bind _compasstrigger (`/Game/Blueprints/BP_QuarterBase.CompassTrigger` _quarter_base_8))
  (bind _compasstrigger_2 (`/Game/Blueprints/BP_QuarterBase.CompassTrigger` _quarter_base))
  (bind _compasstrigger_3 (`/Game/Blueprints/BP_QuarterBase.CompassTrigger` _quarter_base_4))
  (bind _compasstrigger_4 (`/Game/Blueprints/BP_QuarterBase.CompassTrigger` _quarter_base_2))
  (bind _questtrigger_4 (`/Game/Blueprints/BP_QuarterBase.QuestTrigger` _quarter_base_8))
  (bind _tableinteracttrigger_4 (`/Game/Blueprints/BP_QuarterBase.TableInteractTrigger` _quarter_base_8))
  (bind _npctrigger_4 (`/Game/Blueprints/BP_QuarterBase.NPCTrigger` _quarter_base))
  (bind _steertrigger_4 (`/Game/Blueprints/BP_QuarterBase.SteerTrigger` _quarter_base_8))
  (bind _output_get (set `self.CurrentState` Phase))
  (switch `/Game/Blueprints/EM_Phase` _output_get
    (:`NewEnumerator0`
      ;[1 1 1] While at station you can see widgets:
      (`|ExecutionSequence`
        (:`then_0`
          (`PrimitiveComponent.SetCollisionEnabled` _doortrigger "NoCollision")
          (`/Game/Blueprints/BP_QuarterBase.SwitchParentWidget` _quarter_base_6 _doortrigger "NewEnumerator2"))
        (:`then_1`
          (`PrimitiveComponent.SetCollisionEnabled` _npctrigger_4 "QueryAndPhysics")
          (`/Game/Blueprints/BP_QuarterBase.SwitchParentWidget` _quarter_base_6 _npctrigger_4 "NewEnumerator1"))
        (:`then_2`
          (`PrimitiveComponent.SetCollisionEnabled` _questtrigger_3 "QueryAndPhysics")
          (`/Game/Blueprints/BP_QuarterBase.SwitchParentWidget` _quarter_base_6 _questtrigger_3 "NewEnumerator1"))
        (:`then_3`
          (`PrimitiveComponent.SetCollisionEnabled` _tableinteracttrigger_3 "QueryAndPhysics")
          (`/Game/Blueprints/BP_QuarterBase.SwitchParentWidget` _quarter_base_6 _tableinteracttrigger_3 "NewEnumerator1"))
        (:`then_4`
          (`PrimitiveComponent.SetCollisionEnabled` _steertrigger_3 "QueryAndPhysics")
          (`/Game/Blueprints/BP_QuarterBase.SwitchParentWidget` _quarter_base_6 _steertrigger_3 "NewEnumerator1"))
        (:`then_5`
          (`PrimitiveComponent.SetCollisionEnabled` _scenerytrigger_4 "QueryAndPhysics")
          (`/Game/Blueprints/BP_QuarterBase.SwitchParentWidget` _quarter_base_6 _scenerytrigger_4 "NewEnumerator1"))
        (:`then_6`
          (`PrimitiveComponent.SetCollisionEnabled` _compasstrigger_2 "QueryAndPhysics")
          (`/Game/Blueprints/BP_QuarterBase.SwitchParentWidget` _quarter_base_6 _compasstrigger_2 "NewEnumerator1"))
        (:`then_7`
          (`self.PopupText`))))
    (:`NewEnumerator1`
      ;[1 1 1] While moving you can see widgets:
      (`|ExecutionSequence`
        (:`then_0`
          (`PrimitiveComponent.SetCollisionEnabled` _doortrigger_3 "NoCollision")
          (`/Game/Blueprints/BP_QuarterBase.SwitchParentWidget` _quarter_base_5 _doortrigger_3 "NewEnumerator2"))
        (:`then_1`
          (`PrimitiveComponent.SetCollisionEnabled` _npctrigger_2 "QueryAndPhysics")
          (`/Game/Blueprints/BP_QuarterBase.SwitchParentWidget` _quarter_base_5 _npctrigger_2 "NewEnumerator1"))
        (:`then_2`
          (`PrimitiveComponent.SetCollisionEnabled` _questtrigger_2 "QueryAndPhysics")
          (`/Game/Blueprints/BP_QuarterBase.SwitchParentWidget` _quarter_base_5 _questtrigger_2 "NewEnumerator1"))
        (:`then_3`
          (`PrimitiveComponent.SetCollisionEnabled` _tableinteracttrigger_2 "NoCollision")
          (`/Game/Blueprints/BP_QuarterBase.SwitchParentWidget` _quarter_base_5 _tableinteracttrigger_2 "NewEnumerator2"))
        (:`then_4`
          (`PrimitiveComponent.SetCollisionEnabled` _steertrigger_2 "NoCollision")
          (`/Game/Blueprints/BP_QuarterBase.SwitchParentWidget` _quarter_base_5 _steertrigger_2 "NewEnumerator2"))
        (:`then_5`
          (`PrimitiveComponent.SetCollisionEnabled` _scenerytrigger_3 "QueryAndPhysics")
          (`/Game/Blueprints/BP_QuarterBase.SwitchParentWidget` _quarter_base_5 _scenerytrigger_3 "NewEnumerator1"))
        (:`then_6`
          (`PrimitiveComponent.SetCollisionEnabled` _compasstrigger_3 "NoCollision")
          (`/Game/Blueprints/BP_QuarterBase.SwitchParentWidget` _quarter_base_5 _compasstrigger_3 "NewEnumerator2"))))
    (:`NewEnumerator3`
      ;[1 1 1] While Steering you see widgets:
      (`|ExecutionSequence`
        (:`then_0`
          (`PrimitiveComponent.SetCollisionEnabled` _doortrigger_2 "NoCollision")
          (`/Game/Blueprints/BP_QuarterBase.SwitchParentWidget` _quarter_base_3 _doortrigger_2 "NewEnumerator2"))
        (:`then_1`
          (`PrimitiveComponent.SetCollisionEnabled` _npctrigger "NoCollision")
          (`/Game/Blueprints/BP_QuarterBase.SwitchParentWidget` _quarter_base_3 _npctrigger "NewEnumerator2"))
        (:`then_2`
          (`PrimitiveComponent.SetCollisionEnabled` _questtrigger "NoCollision")
          (`/Game/Blueprints/BP_QuarterBase.SwitchParentWidget` _quarter_base_3 _questtrigger "NewEnumerator2"))
        (:`then_3`
          (`PrimitiveComponent.SetCollisionEnabled` _tableinteracttrigger "QueryAndPhysics")
          (`/Game/Blueprints/BP_QuarterBase.SwitchParentWidget` _quarter_base_3 _tableinteracttrigger "NewEnumerator1"))
        (:`then_4`
          (`PrimitiveComponent.SetCollisionEnabled` _steertrigger "QueryAndPhysics")
          (`/Game/Blueprints/BP_QuarterBase.SwitchParentWidget` _quarter_base_3 _steertrigger "NewEnumerator1"))
        (:`then_5`
          (`PrimitiveComponent.SetCollisionEnabled` _scenerytrigger "QueryAndPhysics")
          (`/Game/Blueprints/BP_QuarterBase.SwitchParentWidget` _quarter_base_3 _scenerytrigger "NewEnumerator1"))
        (:`then_6`
          (`PrimitiveComponent.SetCollisionEnabled` _compasstrigger_4 "NoCollision")
          (`/Game/Blueprints/BP_QuarterBase.SwitchParentWidget` _quarter_base_3 _compasstrigger_4 "NewEnumerator2"))
        (:`then_7`
          (`self.PopupText`))))
    (:`NewEnumerator4`
      ;[1 1 1] While accepting / turning in quests you see:
      (`|ExecutionSequence`
        (:`then_0`
          (`PrimitiveComponent.SetCollisionEnabled` _doortrigger_4 "QueryAndPhysics")
          (`/Game/Blueprints/BP_QuarterBase.SwitchParentWidget` _quarter_base_7 _doortrigger_4 "NewEnumerator1"))
        (:`then_1`
          (`PrimitiveComponent.SetCollisionEnabled` _npctrigger_3 "NoCollision")
          (`/Game/Blueprints/BP_QuarterBase.SwitchParentWidget` _quarter_base_7 _npctrigger_3 "NewEnumerator2"))
        (:`then_2`
          (`PrimitiveComponent.SetCollisionEnabled` _questtrigger_4 "QueryAndPhysics")
          (`/Game/Blueprints/BP_QuarterBase.SwitchParentWidget` _quarter_base_7 _questtrigger_4 "NewEnumerator1"))
        (:`then_3`
          (`PrimitiveComponent.SetCollisionEnabled` _tableinteracttrigger_4 "QueryAndPhysics")
          (`/Game/Blueprints/BP_QuarterBase.SwitchParentWidget` _quarter_base_7 _tableinteracttrigger_4 "NewEnumerator1"))
        (:`then_4`
          (`PrimitiveComponent.SetCollisionEnabled` _steertrigger_4 "NoCollision")
          (`/Game/Blueprints/BP_QuarterBase.SwitchParentWidget` _quarter_base_7 _steertrigger_4 "NewEnumerator2"))
        (:`then_5`
          (`PrimitiveComponent.SetCollisionEnabled` _scenerytrigger_2 "QueryAndPhysics")
          (`/Game/Blueprints/BP_QuarterBase.SwitchParentWidget` _quarter_base_7 _scenerytrigger_2 "NewEnumerator1"))
        (:`then_6`
          (`PrimitiveComponent.SetCollisionEnabled` _compasstrigger "NoCollision")
          (`/Game/Blueprints/BP_QuarterBase.SwitchParentWidget` _quarter_base_7 _compasstrigger "NewEnumerator2"))
        (:`then_7`
          (`self.PopupText`))))))