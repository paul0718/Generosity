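; AC_CompassSystem is a component for BP_QuarterBase that manages a compass serving as a random number roller.
; On BeginPlay it caches the owning base, then spawns a BP_Compass at the base's Compass component transform and attaches it to the base.
; RollNumberAndTakeOff picks a number from one to MaxRoll, shows it on the compass text, then calls TakesOff on the base's flow control component.
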(event `self.ReceiveBeginPlay`
  (bind _compass (`/Game/Blueprints/BP_QuarterBase.compass` (`self.QuarterBase`)))
  (`|ExecutionSequence`
    (:`then_0`
      (bind _asbp_quarter_base (cast `/Game/Blueprints/BP_QuarterBase` (`self.GetOwner`)))
      (set `self.QuarterBase` _asbp_quarter_base))
    (:`then_1`
      (bind _returnvalue (`|SpawnActorFromClass` "/Game/Blueprints/BP_Compass.BP_Compass_C" (`KismetMathLibrary.MakeTransform` (`SceneComponent.K2_GetComponentLocation` _compass) (`SceneComponent.K2_GetComponentRotation` _compass)) "Undefined" "MultiplyWithRoot" null null))
      (bind _output_get (set `self.Compass` _returnvalue))
      (`Actor.K2_AttachToActor` _output_get (`self.QuarterBase`) "None" "KeepWorld" "KeepWorld" "KeepWorld" true))))

(fn `RollNumberAndTakeOff`
  (`|ExecutionSequence`
    (:`then_0`
      (bind _output_get (set `self.Roll` (`KismetMathLibrary.RandomIntegerInRange` 1 (`self.MaxRoll`))))
      (`TextRenderComponent.K2_SetText` (`/Game/Blueprints/BP_Compass.Number` (`self.Compass`)) (`KismetTextLibrary.Conv_IntToText` _output_get)))
    (:`then_1`
      (`/Game/Blueprints/AC_FlowControl.Takes off` (`/Game/Blueprints/BP_QuarterBase.AC_FlowControl` (`self.QuarterBase`))))))