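; BP_Steer is a steer actor that plays a timed spin animation with an accompanying Direction component.
; Spin drives a five-second timeline that rotates the root, counter-rotates Direction, pins it above BP_QuarterBase's Steer component, and tracks IsSpinning.
; ReverseSpin plays that timeline backwards.
; Turn180Degree starts a separate arrow timeline that has no outputs wired.
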(event `Spin`
  (bind (_direction _alpha) (`Timeline|5SecondSpin` :!via `PlayFromStart` :!label _label)
    (:`Update`
      (bind _returnvalue (`KismetMathLibrary.RLerp` (`self.0Rotator`) (`self.360Rotator`) _alpha))
      (`SceneComponent.K2_SetRelativeRotation` (`self.DefaultSceneRoot`) _returnvalue false false)
      (`SceneComponent.K2_SetRelativeRotation` (`self.Direction`) (`KismetMathLibrary.NegateRotator` _returnvalue) false false)
      (bind _returnvalue_2 (`GameplayStatics.GetActorOfClass` "/Game/Blueprints/BP_QuarterBase.BP_QuarterBase_C"))
      (`SceneComponent.K2_SetWorldLocation` (`self.Direction`) (+ (`SceneComponent.K2_GetComponentLocation` (`/Game/Blueprints/BP_QuarterBase.Steer` _returnvalue_2)) (0.0 0.0 173.0)) false false)
      (set `self.IsSpinning` true))
    (:`Finished`
      (set `self.IsSpinning` false))))

(event `ReverseSpin`
  (goto _label :!via `Reverse`))

(event `Turn180Degree`
  (`Timeline|5SecondLerpForArrow` :!via `PlayFromStart`))

(fn `UserConstructionScript`)