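; BP_SplineRoad is an actor that moves a Ship component along a spline path built from waypoint actors.
; BeginPlay rebuilds the spline from each waypoint's AC_WayPoint location.
; Tick advances distance by SplineSpeed and places the ship there with height and yaw offsets, optionally looping to the start.
; Space bar toggles movement through a FlipFlop that sets the Stopped flag.
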(event `self.ReceiveBeginPlay`
  (`SplineComponent.ClearSplinePoints` (`self.Spline`) true)
  (for _array_element (`self.WayPointsActors`)
    (`SplineComponent.AddSplinePoint` (`self.Spline`) (`/Game/Blueprints/AC_WayPoint.WayPointLocation` (`self.GetComponentByClass` _array_element "/Game/Blueprints/AC_WayPoint.AC_WayPoint_C")) "World" true))
  (`SplineComponent.UpdateSpline` (`self.Spline`)))

(event `self.ReceiveTick`
  (params (DeltaSeconds :type "Float (single-precision)"))
  (bind _returnvalue (`SplineComponent.GetTransformAtDistanceAlongSpline` (`self.Spline`) (`self.DistanceAlongSpline`) "Local" false))
  (if (not (`self.stopped`))
    (set `self.DistanceAlongSpline` (+ (* DeltaSeconds (`self.SplineSpeed`)) (`self.DistanceAlongSpline`)))
    (`SceneComponent.K2_SetRelativeTransform` (`self.Ship`) (`KismetMathLibrary.MakeTransform` (`KismetMathLibrary.MakeVector` (.x (.location _returnvalue)) (.y (.location _returnvalue)) (+ (.z (.location _returnvalue)) 50.0)) (`KismetMathLibrary.MakeRotator` (.roll (.rotation _returnvalue)) 0.0 (+ (.yaw (.rotation _returnvalue)) -90.0)) (`SceneComponent.RelativeScale3D` (`self.Ship`))) false false)
    (if (`self.loop`)
      (if (> (`self.DistanceAlongSpline`) (`SplineComponent.GetSplineLength` (`self.Spline`)))
        (set `self.DistanceAlongSpline` 0.0)))))

(event `Key|SpaceBar`
  (params (Key :type "Key Structure"))
  (:`Pressed`
    (`/Engine/EditorBlueprintResources/StandardMacros.FlipFlop`
      (:`A`
        (set `self.stopped` true))
      (:`B`
        (set `self.stopped` false)))))

(fn `UserConstructionScript`)