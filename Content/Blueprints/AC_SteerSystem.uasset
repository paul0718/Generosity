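; Actor component that gives a BP_QuarterBase its steering wheel and tracks whether steer mode is active.
; On BeginPlay it spawns a BP_Steer above the owner's Steer component, attaches it and turns it around.
; Turn and switch events spin the wheel unless already spinning, some also updating its Direction text, which FinishSwitch resets to a direction name.
; Entering steer mode also calls TakeOff on the ship controller; quitting only clears the flag.
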(event `self.ReceiveBeginPlay`
  (bind _asbp_quarter_base (cast `/Game/Blueprints/BP_QuarterBase` (`self.GetOwner`)))
  (bind _output_get (set `self.Quarter Base` _asbp_quarter_base))
  (bind _returnvalue (`|SpawnActorFromClass` "/Game/Blueprints/BP_Steer.BP_Steer_C" (`KismetMathLibrary.MakeTransform` (+ (`SceneComponent.K2_GetComponentLocation` (`/Game/Blueprints/BP_QuarterBase.Steer` _output_get)) (0.0 0.0 128.0))) "Undefined" "MultiplyWithRoot" null null))
  (bind _output_get_2 (set `self.Steer` _returnvalue))
  (`Actor.K2_AttachToActor` _output_get_2 (`self.Quarter Base`) "None" "KeepWorld" "KeepWorld" "KeepWorld" true)
  (`SceneComponent.K2_SetRelativeRotation` (`/Game/Blueprints/BP_Steer.DefaultSceneRoot` (`self.Steer`)) (struct :`Yaw` 180.0) false false))

(event `TurnWheel`
  (params (Text :type Text))
  (if (not (`/Game/Blueprints/BP_Steer.IsSpinning` (`self.Steer`)))
    (`/Game/Blueprints/BP_Steer.Spin` (`self.Steer`))
    (`TextRenderComponent.K2_SetText` (`/Game/Blueprints/BP_Steer.Direction` (`self.Steer`)) Text)))

(event `SwitchLine`
  (if (not (`/Game/Blueprints/BP_Steer.IsSpinning` (`self.Steer`)))
    (`/Game/Blueprints/BP_Steer.Spin` (`self.Steer`))
    (`TextRenderComponent.K2_SetText` (`/Game/Blueprints/BP_Steer.Direction` (`self.Steer`)) (`KismetTextLibrary.Conv_NameToText` (`|GetArrayItem` (`self.SwitchLineIndicateName`))))))

(event `FinishSwitch`
  (`TextRenderComponent.K2_SetText` (`/Game/Blueprints/BP_Steer.Direction` (`self.Steer`)) (`KismetTextLibrary.Conv_NameToText` (`|GetArrayItem` (`self.DirectionName`)))))

(event `SwitchLeft`
  (if (not (`/Game/Blueprints/BP_Steer.IsSpinning` (`self.Steer`)))
    (`/Game/Blueprints/BP_Steer.Spin` (`self.Steer`))))

(event `SwitchRight`
  (if (not (`/Game/Blueprints/BP_Steer.IsSpinning` (`self.Steer`)))
    (`/Game/Blueprints/BP_Steer.Spin` (`self.Steer`))))

(fn `Enter Steer Mode`
  (set `self.isInSteerMode` true)
  (`/Game/Blueprints/ShipMovement/AC_ShipController.Take Off` (`/Game/Blueprints/BP_QuarterBase.AC_ShipController` (`self.Quarter Base`))))

(fn `QuitSteerMode`
  (set `self.isInSteerMode` false))