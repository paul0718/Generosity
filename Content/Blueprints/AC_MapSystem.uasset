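; Map system component for BP_QuarterBase that manages the in-world map display and station selection.
; On BeginPlay it spawns a scaled BP_Map at the owner's Map transform, attaches it, and collects the level's tier 0 stations.
; UnlockLine and GrowLine reveal map line segments, while SetDestination forwards to the owner's ship controller.
; Random draws cover tiers 0 and 1, though tier 1 is never filled here; map-mode enter and quit are empty stubs.
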(event `self.ReceiveBeginPlay`
  (`|ExecutionSequence`
    (:`then_0`
      (bind _asbp_quarter_base (cast `/Game/Blueprints/BP_QuarterBase` (`self.GetOwner`))
        (:`then`
          (set `self.QuarterBase` _asbp_quarter_base))
        (:`CastFailed`
          (`KismetSystemLibrary.PrintString` "FATAL ERROR CAST FAILLL" true true (struct :`R` 1.0 :`B` 0.136706 :`A` 1.0)))))
    (:`then_1`
      (bind _returnvalue (`|SpawnActorFromClass` "/Game/Blueprints/BP_Map.BP_Map_C" (`KismetMathLibrary.MakeTransform` (.location (`SceneComponent.K2_GetComponentToWorld` (`/Game/Blueprints/BP_QuarterBase.Map` (`self.QuarterBase`)))) (.rotation (`SceneComponent.K2_GetComponentToWorld` (`/Game/Blueprints/BP_QuarterBase.Map` (`self.QuarterBase`)))) (* (1.0 1.0 1.0) 1.3)) "AlwaysSpawn" "MultiplyWithRoot" null null))
      (bind _output_get (set `self.MapDisplay` _returnvalue))
      (`Actor.K2_AttachToActor` _output_get (`self.QuarterBase`) "None" "KeepWorld" "KeepWorld" "KeepWorld" true))
    (:`then_2`
      (bind _outactors (`GameplayStatics.GetAllActorsOfClass` "/Game/Blueprints/BP_Station.BP_Station_C"))
      (for _array_element _outactors
        (if (== (`/Game/Blueprints/BP_Station.UnlockTier` _array_element) 0)
          (`KismetArrayLibrary.Array_Add` (`self.AvailableStations`) _array_element)))
      (set `self.AvailableTier0Stations` (`self.AvailableStations`)))))

(fn `Draw Random Station With Tier`
  (params (Tier :type Integer))
  (returns (Station :type "/Game/Blueprints/BP_Station Object Reference"))
  (switch `int` Tier
    (:`0`
      (return (`KismetArrayLibrary.Array_Random` (`self.AvailableTier0Stations`))))
    (:`1`
      (return (`KismetArrayLibrary.Array_Random` (`self.AvailableTier1Stations`))))))

(fn `EnterMapMode`)

(fn `Grow Line`
  (params (`Line Subindex` :type Integer))
  (bind _mapdisplay (`self.MapDisplay`))
  (switch `int` `Line Subindex`
    (:`1`
      (`SceneComponent.SetVisibility` (`/Game/Blueprints/BP_Map.Line2-1-X` _mapdisplay) true false))
    (:`2`
      (`SceneComponent.SetVisibility` (`/Game/Blueprints/BP_Map.Line2-2-X` _mapdisplay) true false))
    (:`3`
      (`SceneComponent.SetVisibility` (`/Game/Blueprints/BP_Map.Line2-3-X` _mapdisplay) true false))
    (:`4`
      (`SceneComponent.SetVisibility` (`/Game/Blueprints/BP_Map.Line2-4-X` _mapdisplay) true false))))

(fn `QuitMapMode`)

(fn `SetDestination`
  (params (`Station Name` :type Name))
  (`/Game/Blueprints/ShipMovement/AC_ShipController.Set Destination` (`/Game/Blueprints/BP_QuarterBase.AC_ShipController` (`self.QuarterBase`)) `Station Name`))

(fn `Unlock Line`
  (params (`Line Tier` :type Integer) (`Line Index` :type Integer))
  (bind _mapdisplay (`self.MapDisplay`))
  (bind _mapdisplay_2 (`self.MapDisplay`))
  (switch `int` `Line Tier`
    (:`1`
      (`|ExecutionSequence`
        (:`then_0`
          ;[1 1 1] Make Visible
          (switch `int` (`local.Line Index`)
            (:`1`
              (`SceneComponent.SetVisibility` (`/Game/Blueprints/BP_Map.Line1-1` _mapdisplay_2) true false))
            (:`2`
              (`SceneComponent.SetVisibility` (`/Game/Blueprints/BP_Map.Line1-2` _mapdisplay_2) true false))
            (:`3`
              (`SceneComponent.SetVisibility` (`/Game/Blueprints/BP_Map.Line1-3` _mapdisplay_2) true false))
            (:`4`
              (`SceneComponent.SetVisibility` (`/Game/Blueprints/BP_Map.Line1-4` _mapdisplay_2) true false))))))
    (:`2`
      (`|ExecutionSequence`
        (:`then_0`
          (switch `int` (`local.Line Index`)
            (:`1`
              (`SceneComponent.SetVisibility` (`/Game/Blueprints/BP_Map.Line2-1-0` _mapdisplay) true false))
            (:`2`
              (`SceneComponent.SetVisibility` (`/Game/Blueprints/BP_Map.Line2-2-0` _mapdisplay) true false))
            (:`3`
              (`SceneComponent.SetVisibility` (`/Game/Blueprints/BP_Map.Line2-3-0` _mapdisplay) true false))
            (:`4`
              (`SceneComponent.SetVisibility` (`/Game/Blueprints/BP_Map.Line2-4-0` _mapdisplay) true false))))))
    (:`3`
      (`SceneComponent.SetVisibility` (`/Game/Blueprints/BP_Map.Line3` (`self.MapDisplay`)) true false))))