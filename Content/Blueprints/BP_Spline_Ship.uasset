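; BP_Spline_Ship is a spline path actor that drives the level's BP_QuarterBase along its route, apparently as a moving ship.
; BeginPlay finds that actor by class, then Tick advances a distance at SplineSpeed unless Stopped.
; The spline's local-space transform is applied to the base's root as a relative transform, with height and yaw offsets and no spline pitch.
; When Loop is set, distance resets past the spline's end.
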(event `self.ReceiveTick`
  (params (DeltaSeconds :type "Float (single-precision)"))
  (bind _returnvalue (`SplineComponent.GetTransformAtDistanceAlongSpline` (`self.Spline`) (`self.DistanceAlongSpline`) "Local" false))
  (if (not (`self.stopped`))
    (set `self.DistanceAlongSpline` (+ (* DeltaSeconds (`self.SplineSpeed`)) (`self.DistanceAlongSpline`)))
    (`SceneComponent.K2_SetRelativeTransform` (`Actor.RootComponent` (`self.BP_QuarterBase`)) (`KismetMathLibrary.MakeTransform` (`KismetMathLibrary.MakeVector` (.x (.location _returnvalue)) (.y (.location _returnvalue)) (+ (.z (.location _returnvalue)) 50.0)) (`KismetMathLibrary.MakeRotator` (.roll (.rotation _returnvalue)) 0.0 (+ (.yaw (.rotation _returnvalue)) -90.0)) (`SceneComponent.RelativeScale3D` (`Actor.RootComponent` (`self.BP_QuarterBase`)))) false false)
    (if (`self.loop`)
      (if (> (`self.DistanceAlongSpline`) (`SplineComponent.GetSplineLength` (`self.Spline`)))
        (set `self.DistanceAlongSpline` 0.0)))))

(event `self.ReceiveBeginPlay`
  (bind _returnvalue (`GameplayStatics.GetActorOfClass` "/Game/Blueprints/BP_QuarterBase.BP_QuarterBase_C"))
  (set `self.BP_QuarterBase` _returnvalue))

(fn `UserConstructionScript`)