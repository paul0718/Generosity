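; Station actor where ships land and take off along the spline lines of BP_NaviSystem.
; On BeginPlay it finds lines passing within 100 units of its detect point, caches each one's input key and a shared world location, and flags itself as a transfer if several match.
; Landing and takeoff splines are anchored at the landing zone, with functions to set their outer ends to detach and attach points.
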(event `self.ReceiveBeginPlay`
  (bind _returnvalue (`SceneComponent.K2_GetComponentLocation` (`self.LocationOnLineDetectPoint`)))
  (`|ExecutionSequence`
    (:`then_0`
      (set `self.WorldLocationLanding` (`SceneComponent.K2_GetComponentLocation` (`self.LandingZone`))))
    (:`then_1`
      (bind _returnvalue_2 (`GameplayStatics.GetActorOfClass` "/Game/Blueprints/BP_NaviSystem.BP_NaviSystem_C"))
      (set `self.NaviSystem` _returnvalue_2))
    (:`then_2`
      (for (_array_element _array_index) (`/Game/Blueprints/BP_NaviSystem.Lines` (`self.NaviSystem`))
        (bind _spline (`/Game/Blueprints/BP_Spline_Road.Spline` _array_element))
        (bind _returnvalue_3 (`SplineComponent.FindInputKeyClosestToWorldLocation` _spline _returnvalue))
        (bind _returnvalue_location (`KismetMathLibrary.BreakTransform` (`SplineComponent.GetTransformAtSplineInputKey` _spline _returnvalue_3 "World" false)))
        (if (<= (`KismetMathLibrary.Vector_Distance` _returnvalue_location _returnvalue) 100.0)
          (`BlueprintMapLibrary.Map_Add` (`self.InputKeysOnLines`) _array_index _returnvalue_3)
          ;[1 1 1] Assuming World Locations On Different Lines for the Same Station are Exactly the Same, Preventing Ship Teleporting
          (set `self.WorldLocationOnLines` _returnvalue_location))))
    (:`then_3`
      (if (> (`BlueprintMapLibrary.Map_Length` (`self.InputKeysOnLines`)) 1)
        (set `self.IsTransfer` true)))
    (:`then_4`
      (`SplineComponent.SetLocationAtSplinePoint` (`self.TakeOffTrack`) 0 (`self.WorldLocationLanding`) "World" true)
      (`SplineComponent.SetLocationAtSplinePoint` (`self.LandingTrack`) 1 (`self.WorldLocationLanding`) "World" true))))

(fn `SetLandingTrack`
  (params (DetachFromWorld :type "Vector Structure"))
  (`SplineComponent.SetLocationAtSplinePoint` (`self.LandingTrack`) 0 DetachFromWorld "World" true))

(fn `SetTakeOffTrack`
  (params (AttachToWorld :type "Vector Structure"))
  (`SplineComponent.SetLocationAtSplinePoint` (`self.TakeOffTrack`) 1 AttachToWorld "World" true))

(fn `UserConstructionScript`)