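; Quarters base actor with a swinging door, a table camera view and proximity interaction prompts.
; Key 0 toggles the door through a timeline-driven yaw rotation.
; Key 9 toggles the first-person character's camera to and from TableView when CanSwitch allows.
; Four trigger volumes share SwitchParentWidget, which finds sibling prompt widgets and shows the parent component's name with an E-key icon, reverting to an indicator point on exit.
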(event `Key|Zero`
  (params (Key :type "Key Structure"))
  (:`Pressed`
    (`/Engine/EditorBlueprintResources/StandardMacros.FlipFlop`
      (:`A`
        (`self.OpenDoor`))
      (:`B`
        (`self.CloseDoor`)))))

(event `Key|Nine`
  (params (Key :type "Key Structure"))
  (:`Pressed`
    (bind _returnvalue (`GameplayStatics.GetActorOfClass` "/Game/FirstPerson/Blueprints/BP_FirstPersonCharacter.BP_FirstPersonCharacter_C"))
    (if (`/Game/FirstPerson/Blueprints/BP_FirstPersonCharacter.canSwitch` _returnvalue)
      (`/Engine/EditorBlueprintResources/StandardMacros.FlipFlop`
        (:`A`
          (`/Game/FirstPerson/Blueprints/BP_FirstPersonCharacter.SwitchCameraToPoint` _returnvalue (`SceneComponent.K2_GetComponentToWorld` (`self.TableView`))))
        (:`B`
          (`/Game/FirstPerson/Blueprints/BP_FirstPersonCharacter.SwitchCameraBack` _returnvalue))))))

(event `OpenDoor`
  (bind (_direction _doorfloat) (`Timeline|OpentheDoorTimeline` :!via `PlayFromStart` :!label _label)
    (:`Update`
      (`SceneComponent.K2_SetRelativeRotation` (`self.DoorSelf`) (`KismetMathLibrary.MakeRotator` 0.0 0.0 (+ (`KismetMathLibrary.Lerp` 0.0 90.0 _doorfloat) -180.0)) false false))))

(event `CloseDoor`
  (goto _label :!via `Reverse`))

(event `self.InteractTrigger.OnComponentBeginOverlap`
  (params (OverlappedComponent :type "PrimitiveComponent Object Reference") (OtherActor :type "Actor Object Reference") (OtherComp :type "PrimitiveComponent Object Reference") (OtherBodyIndex :type Integer) (bFromSweep :type Boolean) (SweepResult :type "HitResult Structure (by ref)"))
  (`self.SwitchParentWidget` OverlappedComponent true))

(event `self.InteractTrigger.OnComponentEndOverlap`
  (params (OverlappedComponent :type "PrimitiveComponent Object Reference") (OtherActor :type "Actor Object Reference") (OtherComp :type "PrimitiveComponent Object Reference") (OtherBodyIndex :type Integer))
  (`self.SwitchParentWidget` OverlappedComponent))

(event `self.InteractTrigger1.OnComponentBeginOverlap`
  (params (OverlappedComponent :type "PrimitiveComponent Object Reference") (OtherActor :type "Actor Object Reference") (OtherComp :type "PrimitiveComponent Object Reference") (OtherBodyIndex :type Integer) (bFromSweep :type Boolean) (SweepResult :type "HitResult Structure (by ref)"))
  (`self.SwitchParentWidget` OverlappedComponent true))

(event `self.InteractTrigger1.OnComponentEndOverlap`
  (params (OverlappedComponent :type "PrimitiveComponent Object Reference") (OtherActor :type "Actor Object Reference") (OtherComp :type "PrimitiveComponent Object Reference") (OtherBodyIndex :type Integer))
  (`self.SwitchParentWidget` OverlappedComponent))

(event `self.InteractTrigger2.OnComponentBeginOverlap`
  (params (OverlappedComponent :type "PrimitiveComponent Object Reference") (OtherActor :type "Actor Object Reference") (OtherComp :type "PrimitiveComponent Object Reference") (OtherBodyIndex :type Integer) (bFromSweep :type Boolean) (SweepResult :type "HitResult Structure (by ref)"))
  (`self.SwitchParentWidget` OverlappedComponent true))

(event `self.InteractTrigger2.OnComponentEndOverlap`
  (params (OverlappedComponent :type "PrimitiveComponent Object Reference") (OtherActor :type "Actor Object Reference") (OtherComp :type "PrimitiveComponent Object Reference") (OtherBodyIndex :type Integer))
  (`self.SwitchParentWidget` OverlappedComponent))

(event `self.InteractTrigger3.OnComponentBeginOverlap`
  (params (OverlappedComponent :type "PrimitiveComponent Object Reference") (OtherActor :type "Actor Object Reference") (OtherComp :type "PrimitiveComponent Object Reference") (OtherBodyIndex :type Integer) (bFromSweep :type Boolean) (SweepResult :type "HitResult Structure (by ref)"))
  (`self.SwitchParentWidget` OverlappedComponent true))

(event `self.InteractTrigger3.OnComponentEndOverlap`
  (params (OverlappedComponent :type "PrimitiveComponent Object Reference") (OtherActor :type "Actor Object Reference") (OtherComp :type "PrimitiveComponent Object Reference") (OtherBodyIndex :type Integer))
  (`self.SwitchParentWidget` OverlappedComponent))

(fn `SwitchParentWidget`
  (params (trigger :type "SceneComponent Object Reference") (On :type Boolean))
  (for _array_element (`SceneComponent.GetChildrenComponents` (`|GetArrayItem` (`SceneComponent.GetParentComponents` trigger)) false)
    (if (== (`GameplayStatics.GetObjectClass` _array_element) "/Script/UMG.WidgetComponent")
      (bind _aswidget_component (cast `WidgetComponent` _array_element))
      (if (`local.On`)
        (bind _asw_interactive_prompt (cast `/Game/Blueprints/W_InteractivePrompt` (`WidgetComponent.GetWidget` _aswidget_component)))
        (set `/Game/Blueprints/W_InteractivePrompt.ShownText` (`KismetTextLibrary.Conv_StringToText` (`KismetSystemLibrary.GetObjectName` (`|GetArrayItem` (`SceneComponent.GetParentComponents` (`local.trigger`))))) _asw_interactive_prompt)
        (set `/Game/Blueprints/W_InteractivePrompt.Image` "/Game/Input_Prompts_Pack/Keyboard_Mouse/White/T_E_Key_White.T_E_Key_White" _asw_interactive_prompt)
        (else
          (bind _asw_interactive_prompt_2 (cast `/Game/Blueprints/W_InteractivePrompt` (`WidgetComponent.GetWidget` _aswidget_component)))
          (set `/Game/Blueprints/W_InteractivePrompt.ShownText` "" _asw_interactive_prompt_2)
          (set `/Game/Blueprints/W_InteractivePrompt.Image` "/Game/Textures/IndicatorPoint.IndicatorPoint" _asw_interactive_prompt_2))))))

(fn `UserConstructionScript`)