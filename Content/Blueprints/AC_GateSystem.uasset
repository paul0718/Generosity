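; Actor component for a BP_QuarterBase owner that toggles a gate mode around the current tile quest.
; It caches the owner on BeginPlay; entering the mode disables the door trigger's collision and, if CurrentTileQuest is valid, shows its check and X marks with collision enabled.
; Quitting switches both marks off through the owner's quest manager but leaves the door trigger untouched.
; CurrentTileQuest is never assigned within this component.
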(event `self.ReceiveBeginPlay`
  (bind _asbp_quarter_base (cast `/Game/Blueprints/BP_QuarterBase` (`self.GetOwner`)))
  (set `self.QuarterBase` _asbp_quarter_base))

(fn `EnterGateMode`
  (bind _currenttilequest (`self.CurrentTileQuest`))
  (`|ExecutionSequence`
    (:`then_0`
      (`PrimitiveComponent.SetCollisionEnabled` (`/Game/Blueprints/BP_QuarterBase.DoorTrigger` (`self.QuarterBase`)) "NoCollision"))
    (:`then_1`
      (`/Engine/EditorBlueprintResources/StandardMacros.IsValid` (`self.CurrentTileQuest`)
        (:`Is Valid`
          (`|ExecutionSequence`
            (:`then_0`
              (`SceneComponent.SetVisibility` (`/Game/Blueprints/BP_Quest.CheckMark` _currenttilequest) true false)
              (`PrimitiveComponent.SetCollisionEnabled` (`/Game/Blueprints/BP_Quest.CheckMarkCollision` _currenttilequest) "QueryAndPhysics"))
            (:`then_1`
              (`SceneComponent.SetVisibility` (`/Game/Blueprints/BP_Quest.XMark` _currenttilequest) true false)
              (`PrimitiveComponent.SetCollisionEnabled` (`/Game/Blueprints/BP_Quest.XMarkCollision` _currenttilequest) "QueryAndPhysics"))))))))

(fn `QuitGateMode`
  (`/Engine/EditorBlueprintResources/StandardMacros.IsValid` (`self.CurrentTileQuest`)
    (:`Is Valid`
      (`/Game/Blueprints/AC_QuestManager.CheckMarksSwitchState` (`/Game/Blueprints/BP_QuarterBase.AC_QuestManager` (`self.QuarterBase`)) (`self.CurrentTileQuest`) false false))))