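; BI_Quest_T0_1 is a quest Blueprint that sets its destination to the station named Scorchwick.
; On BeginPlay it runs the parent logic, gets the BP_QuarterBase actor, and searches the MajorStations list on its ACMapSystem component for that name.
; The match is stored in DestinationStation; the construction script only calls the parent, and the Tick and overlap events are disabled.
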(event `self.ReceiveBeginPlay`
  (`parent.ReceiveBeginPlay`)
  (bind _returnvalue (`GameplayStatics.GetActorOfClass` "/Game/Blueprints/BP_QuarterBase.BP_QuarterBase_C"))
  (for _array_element (`/Game/Blueprints/AC_MapSystem.MajorStations` (`/Game/Blueprints/BP_QuarterBase.AC_MapSystem` _returnvalue))
    (if (== (`/Game/Blueprints/BP_Station.Name` _array_element) "Scorchwick")
      (set `self.Destination Station` _array_element))))

(fn `UserConstructionScript`
  (`parent.UserConstructionScript`))