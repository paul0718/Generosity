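; Quest manager component for BP_QuarterBase that spawns station quests, holds them in a physical quest log and tracks player reputation.
; Reputation bands weight tier 1/2 draws of delivery or escort quests (submission only prints), while Tier 0 spawns separately by progress.
; Logged quests fill free slots in a transform-keyed map, and round passes check them against inventory.
; Quest mode toggles check/X marks by status and flow state; completion awards reputation.
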(event `self.ReceiveBeginPlay`
  (bind _asbp_quarter_base (cast `/Game/Blueprints/BP_QuarterBase` (`self.GetOwner`)))
  (set `self.QuarterBase` _asbp_quarter_base)
  (bind _keys (`BlueprintMapLibrary.Map_Keys` (`self.QuestRelativeLocations`)))
  (for _array_element _keys
    (`BlueprintMapLibrary.Map_Add` (`self.QuestRelativeLocations`) _array_element)))

(fn `Add Quest to Log`
  (params (Quest :type "/Game/Blueprints/BP_Quest Object Reference"))
  (if (< (`KismetArrayLibrary.Array_Length` (`self.QuestList`)) (`self.QuestMaxSize`))
    (bind _keys (`BlueprintMapLibrary.Map_Keys` (`self.QuestRelativeLocations`)))
    (for _array_element _keys
      (if (not (`KismetSystemLibrary.IsValid` (`BlueprintMapLibrary.Map_Find` (`self.QuestRelativeLocations`) _array_element)))
        (`SceneComponent.K2_SetWorldTransform` (`Actor.RootComponent` (`local.Quest`)) (`KismetMathLibrary.ComposeTransforms` _array_element (`SceneComponent.K2_GetComponentToWorld` (`/Game/Blueprints/BP_QuarterBase.QuestLog` (`self.QuarterBase`)))) false false)
        (`KismetArrayLibrary.Array_Add` (`self.QuestList`) (`local.Quest`))
        (`BlueprintMapLibrary.Map_Add` (`self.QuestRelativeLocations`) _array_element (`local.Quest`))
        (break)))
    (`|ExecutionSequence`
      (:`then_0`
        (`Actor.K2_AttachToComponent` (`local.Quest`) (`/Game/Blueprints/BP_QuarterBase.QuestLog` (`self.QuarterBase`)) "None" "KeepWorld" "KeepWorld" "KeepWorld" true)
        (return)))
    (else
      (`self.Remove Quest` Quest))))

(fn `CheckMarksSwitchState`
  (params (Quest :type "/Game/Blueprints/BP_Quest Object Reference") (`Check State` :type Boolean) (`X State` :type Boolean))
  (bind _checkmarkcollision (`/Game/Blueprints/BP_Quest.CheckMarkCollision` Quest))
  (bind _xmarkcollision (`/Game/Blueprints/BP_Quest.XMarkCollision` Quest))
  (`|ExecutionSequence`
    (:`then_0`
      (`SceneComponent.SetVisibility` (`/Game/Blueprints/BP_Quest.CheckMark` Quest) (`local.Check State`) false)
      (if (`local.Check State`)
        (`PrimitiveComponent.SetCollisionEnabled` _checkmarkcollision "QueryAndPhysics")
        (else
          (`PrimitiveComponent.SetCollisionEnabled` _checkmarkcollision "NoCollision"))))
    (:`then_1`
      (`SceneComponent.SetVisibility` (`/Game/Blueprints/BP_Quest.XMark` Quest) (`local.X State`) false)
      (if (`local.X State`)
        (`PrimitiveComponent.SetCollisionEnabled` _xmarkcollision "QueryAndPhysics")
        (else
          (`PrimitiveComponent.SetCollisionEnabled` _xmarkcollision "NoCollision"))))))

(fn `Complete Quest`
  (params (`BP Quest` :type "/Game/Blueprints/BP_Quest Object Reference"))
  (set `self.Reputation` (+ (`self.Reputation`) (`/Game/Blueprints/BP_Quest.ReputationReward` `BP Quest`)))
  (`self.SetReputationStatus`)
  (`self.Remove Quest` (`local.BP Quest`)))

(fn `Construct and Spawn Tier 0 To Station`
  (returns (`Quest Name / Error` :type Name))
  (locals (`Spawned Quest` :type "/Game/Blueprints/BP_Quest Object Reference"))
  (bind _spawned_quest (`local.Spawned Quest`))
  (switch `int` (`self.Tier0Progress`)
    (:`0`
      (`|ExecutionSequence`
        (:`then_0`
          (bind _returnvalue (`|SpawnActorFromClass` "/Game/Blueprints/QuestBI/BI_Quest_T0_1.BI_Quest_T0_1_C" (`KismetMathLibrary.MakeTransform` (+ (`SceneComponent.K2_GetComponentLocation` (`/Game/Blueprints/BP_QuarterBase.QuestGiving` (`self.QuarterBase`))) (0.0 0.0 0.0)) (struct :`Pitch` -90.0 :`Yaw` -180.0 :`Roll` -110.0) (2.0 2.0 2.0)) "Undefined" "MultiplyWithRoot" null null))
          (bind _output_get (set `local.Spawned Quest` _returnvalue))
          (`Actor.K2_AttachToActor` _output_get (`self.QuarterBase`) "None" "KeepWorld" "KeepWorld" "KeepWorld" true)
          (`SceneComponent.K2_SetRelativeRotation` (`/Game/Blueprints/BP_Quest.DefaultSceneRoot` (`local.Spawned Quest`)) (`SceneComponent.RelativeRotation` (`/Game/Blueprints/BP_QuarterBase.QuestGiving` (`self.QuarterBase`))) false false))
        (:`then_1`
          (set `/Game/Blueprints/AC_GateSystem.CurrentTileQuest` (`local.Spawned Quest`) (`/Game/Blueprints/BP_QuarterBase.AC_GateSystem` (`self.QuarterBase`))))
        (:`then_2`
          (set `self.ConstructedQuest` _spawned_quest)
          (return (`/Game/Blueprints/BP_Quest.QuestName` _spawned_quest)))))))

(fn `ConstructAndSpawnClassToStation`
  (params (`Quest Class` :type "/Game/Blueprints/BP_Quest Class Reference") (QuestTier :type Integer) (Station :type "/Game/Blueprints/BP_Station Object Reference"))
  (returns (`Quest Name / Error` :type Name))
  (locals (SpawnedQuest :type "/Game/Blueprints/BP_Quest Object Reference"))
  (bind _spawnedquest (`local.SpawnedQuest`))
  (`|ExecutionSequence`
    (:`then_0`
      (bind _returnvalue (`|SpawnActorFromClass` `Quest Class` (`KismetMathLibrary.MakeTransform` (+ (`SceneComponent.K2_GetComponentLocation` (`/Game/Blueprints/BP_QuarterBase.QuestGiving` (`self.QuarterBase`))) (0.0 0.0 0.0)) (struct :`Pitch` -90.0 :`Yaw` -180.0 :`Roll` -110.0) (2.0 2.0 2.0)) "Undefined" "MultiplyWithRoot" null null))
      (bind _output_get (set `local.SpawnedQuest` _returnvalue))
      (`Actor.K2_AttachToActor` _output_get (`self.QuarterBase`) "None" "KeepWorld" "KeepWorld" "KeepWorld" true)
      (`SceneComponent.K2_SetRelativeRotation` (`/Game/Blueprints/BP_Quest.DefaultSceneRoot` (`local.SpawnedQuest`)) (`SceneComponent.RelativeRotation` (`/Game/Blueprints/BP_QuarterBase.QuestGiving` (`self.QuarterBase`))) false false))
    (:`then_1`
      (set `/Game/Blueprints/AC_GateSystem.CurrentTileQuest` (`local.SpawnedQuest`) (`/Game/Blueprints/BP_QuarterBase.AC_GateSystem` (`self.QuarterBase`))))
    (:`then_2`
      (bind _station (`/Game/Blueprints/AC_MapSystem.Draw Random Station With Tier` (`/Game/Blueprints/BP_QuarterBase.AC_MapSystem` (`self.QuarterBase`)) (- (`local.QuestTier`) 1)))
      (`/Game/Blueprints/BP_Quest.ConstructQuest` (`local.SpawnedQuest`) _station)
      (set `self.ConstructedQuest` _spawnedquest)
      (return (`/Game/Blueprints/BP_Quest.QuestName` _spawnedquest)))))

(fn `Draw Quest At Station`
  (switch `/Game/Blueprints/EM_ReputationClass` (`self.ReputationLevel`)
    (:`NewEnumerator0`
      (if (<= (`KismetMathLibrary.RandomIntegerInRange` 1 100) 99)
        (`self.Draw Quest Of Tier` 1)
        (else
          (`self.Draw Quest Of Tier` 2))))
    (:`NewEnumerator1`
      (if (<= (`KismetMathLibrary.RandomIntegerInRange` 1 100) 70)
        (`self.Draw Quest Of Tier` 1)
        (else
          (`self.Draw Quest Of Tier` 2))))
    (:`NewEnumerator2`
      (if (<= (`KismetMathLibrary.RandomIntegerInRange` 1 100) 50)
        (`self.Draw Quest Of Tier` 1)
        (else
          (`self.Draw Quest Of Tier` 2))))
    (:`NewEnumerator3`
      (if (<= (`KismetMathLibrary.RandomIntegerInRange` 1 100) 20)
        (`self.Draw Quest Of Tier` 1)
        (else
          (`self.Draw Quest Of Tier` 2))))))

(fn `Draw Quest Of Tier`
  (params (Tier :type Integer))
  (switch `int` (`KismetMathLibrary.RandomIntegerInRange` 0 2)
    (:`0`
      (`self.ConstructAndSpawnClassToStation` "/Game/Blueprints/QuestBI/BI_QuestT1_Delivery.BI_QuestT1_Delivery_C" (`local.Tier`) (`/Game/Blueprints/ShipMovement/AC_ShipController.AtStation` (`/Game/Blueprints/BP_QuarterBase.AC_ShipController` (`self.QuarterBase`)))))
    (:`1`
      (`KismetSystemLibrary.PrintString` "Submission occured!!" true true (struct :`R` 1.0 :`G` 0.756409 :`A` 1.0) 20.0 "Quest"))
    (:`2`
      (`self.ConstructAndSpawnClassToStation` "/Game/Blueprints/QuestBI/BI_QuestT1_Escort.BI_QuestT1_Escort_C" (`local.Tier`) (`/Game/Blueprints/ShipMovement/AC_ShipController.AtStation` (`/Game/Blueprints/BP_QuarterBase.AC_ShipController` (`self.QuarterBase`)))))))

(fn `Enter QuestMode`
  (`|ExecutionSequence`
    (:`then_0`
      (`PrimitiveComponent.SetCollisionEnabled` (`/Game/Blueprints/BP_QuarterBase.QuestTrigger` (`self.QuarterBase`)) "NoCollision"))
    (:`then_1`
      (for _array_element (`self.QuestList`)
        (`|ExecutionSequence`
          (:`then_0`
            (switch `/Game/Blueprints/EM_QuestStatus` (`/Game/Blueprints/BP_Quest.Status` _array_element)
              (:`NewEnumerator0`
                (`self.CheckMarksSwitchState` _array_element false true :!label _label))
              (:`NewEnumerator1`
                (switch `/Game/Blueprints/EM_Phase` (`/Game/Blueprints/AC_FlowControl.CurrentState` (`/Game/Blueprints/BP_QuarterBase.AC_FlowControl` (`self.QuarterBase`)))
                  (:`NewEnumerator0`
                    (`self.CheckMarksSwitchState` _array_element true :!label _label_2))
                  (:`NewEnumerator1`
                    (`self.CheckMarksSwitchState` _array_element :!label _label_3))
                  (:`NewEnumerator3`
                    (goto _label_3))
                  (:`NewEnumerator4`
                    (goto _label_2))))
              (:`NewEnumerator2`
                (goto _label))))
          (:`then_1`
            (if (== (`/Game/Blueprints/BP_Quest.Tier` _array_element) 0)
              (`SceneComponent.SetVisibility` (`/Game/Blueprints/BP_Quest.XMark` _array_element) false false)
              (`PrimitiveComponent.SetCollisionEnabled` (`/Game/Blueprints/BP_Quest.XMarkCollision` _array_element) "NoCollision"))))))))

(fn `Pass Round for Quests`
  (for _array_element (`self.QuestList`)
    (`/Game/Blueprints/BP_Quest.PassRound` _array_element)
    (bind _statustext (`/Game/Blueprints/BP_Quest.Check Quest Status` _array_element (`/Game/Blueprints/AC_Inventory.InventoryMap` (`/Game/Blueprints/BP_QuarterBase.AC_Inventory` (`self.QuarterBase`)))))
    (`KismetSystemLibrary.PrintString` (`|GetEnumeratorNameAsString` _statustext) true true (struct :`R` 1.0 :`G` 0.875824 :`A` 1.0) 50.0)))

(fn `Quit QuestMode`
  (for _array_element (`self.QuestList`)
    (`|ExecutionSequence`
      (:`then_0`
        (`SceneComponent.SetVisibility` (`/Game/Blueprints/BP_Quest.CheckMark` _array_element) false false))
      (:`then_1`
        (`SceneComponent.SetVisibility` (`/Game/Blueprints/BP_Quest.XMark` _array_element) false false))
      (:`then_2`
        (`PrimitiveComponent.SetCollisionEnabled` (`/Game/Blueprints/BP_Quest.CheckMarkCollision` _array_element) "NoCollision"))
      (:`then_3`
        (`PrimitiveComponent.SetCollisionEnabled` (`/Game/Blueprints/BP_Quest.XMarkCollision` _array_element) "NoCollision")))))

(fn `Remove Quest`
  (params (`Quest to be Removed` :type "/Game/Blueprints/BP_Quest Object Reference"))
  (bind _keys (`BlueprintMapLibrary.Map_Keys` (`self.QuestRelativeLocations`)))
  (bind (_arrayindex _arrayelement) (`/Engine/EditorBlueprintResources/StandardMacros.ReverseForEachLoop` _keys)
    (:`LoopBody`
      (if (== (`BlueprintMapLibrary.Map_Find` (`self.QuestRelativeLocations`) _arrayelement) (`local.Quest to be Removed`))
        (`BlueprintMapLibrary.Map_Add` (`self.QuestRelativeLocations`) _arrayelement)))
    (:`Completed`
      (`KismetArrayLibrary.Array_RemoveItem` (`self.QuestList`) (`local.Quest to be Removed`))
      (`Actor.K2_DestroyActor` (`local.Quest to be Removed`)))))

(fn `SetReputationStatus`
  (if (< (`self.Reputation`) 100)
    (set `self.ReputationLevel` "NewEnumerator0")
    (elif (< (`self.Reputation`) 200)
      (set `self.ReputationLevel` "NewEnumerator1")
      (elif (< (`self.Reputation`) 300)
        (set `self.ReputationLevel` "NewEnumerator2")
        (else
          (set `self.ReputationLevel` "NewEnumerator3"))))))