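; Ship controller component that drives its owning actor along the current line's spline each tick, with debug keys toggling direction and stop.
; MoveAlongSpline advances distance by speed, applies spline yaw over the initial rotation with a reverse flip, then wraps on loops or stops at open ends.
; An unfinished TakeOff, never called from the event graph, sets up a station take-off track joining the line.
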(event `Key|Up`
  (params (Key :type "Key Structure"))
  ;[1 1 1] Reverse On Track
  (:`Pressed`
    (`/Engine/EditorBlueprintResources/StandardMacros.FlipFlop`
      (:`A`
        (set `self.IsForwardOnSpline` false))
      (:`B`
        (set `self.IsForwardOnSpline` true)))))

(event `Key|Equals`
  (params (Key :type "Key Structure"))
  ;[1 1 1] Stop Logic
  (:`Pressed`
    (`/Engine/EditorBlueprintResources/StandardMacros.FlipFlop`
      (:`A`
        (set `self.StopFollow` true))
      (:`B`
        (set `self.StopFollow` false)))))

(event `self.ReceiveBeginPlay`
  (bind _returnvalue (`GameplayStatics.GetActorOfClass` "/Game/Blueprints/BP_NaviSystem.BP_NaviSystem_C"))
  (set `self.NaviSystem` _returnvalue)
  (set `self.CurrentSpline` (`/Game/Blueprints/BP_Spline_Road.Spline` (`self.CurrentLine`)))
  (bind _output_get (set `self.ShipActor` (`self.GetOwner`)))
  (set `self.InitialWorldRotation` (`Actor.K2_GetActorRotation` _output_get)))

(event `self.ReceiveTick`
  (params (DeltaSeconds :type "Float (single-precision)"))
  (if (not (`self.StopFollow`))
    (`self.MoveAlongSpline` (`/Game/Blueprints/BP_Spline_Road.Spline` (`self.CurrentLine`)) (`self.ShipActor`))))

(fn `MoveAlongSpline`
  (params (SplineToFollow :type "SplineComponent Object Reference") (ShipActor :type "Actor Object Reference"))
  (bind _splinetofollow (`local.SplineToFollow`))
  (bind _distancealongspline (`self.DistanceAlongSpline`))
  (bind (_initialworldrotation_roll _initialworldrotation_pitch _initialworldrotation_yaw) (`KismetMathLibrary.BreakRotator` (`self.InitialWorldRotation`)))
  (bind _distancealongspline_2 (`self.DistanceAlongSpline`))
  (bind _splinetofollow_2 (`local.SplineToFollow`))
  (bind _returnvalue (`SplineComponent.GetSplineLength` _splinetofollow_2))
  (bind (_returnvalue_roll _returnvalue_pitch _returnvalue_yaw) (`KismetMathLibrary.BreakRotator` (`SplineComponent.GetRotationAtDistanceAlongSpline` _splinetofollow _distancealongspline "World")))
  (set `self.DistanceAlongSpline` (+ (* (* (`GameplayStatics.GetWorldDeltaSeconds`) (`self.Speed`)) (`self.FwdBwd`)) (`self.DistanceAlongSpline`)))
  ;[1 1 1] rotate horizontally based on move direction and spline
  (`Actor.K2_SetActorLocationAndRotation` (`self.ShipActor`) (`SplineComponent.GetLocationAtDistanceAlongSpline` _splinetofollow _distancealongspline "World") (`KismetMathLibrary.MakeRotator` _initialworldrotation_roll _initialworldrotation_pitch (+ (+ _initialworldrotation_yaw _returnvalue_yaw) (* (- 1.0 (`KismetMathLibrary.Conv_BoolToDouble` (`self.IsForwardOnSpline`))) 180.0))) false false)
  ;[1 1 1] Clamp to [0, length] so it works on loops and reverse directions
  (if (`SplineComponent.IsClosedLoop` _splinetofollow_2)
    (set `self.DistanceAlongSpline` (mod (+ (mod (`self.DistanceAlongSpline`) _returnvalue) _returnvalue) _returnvalue))
    (elif (or (>= _distancealongspline_2 _returnvalue) (<= _distancealongspline_2 0.0))
      (set `self.DistanceAlongSpline` (`KismetMathLibrary.FClamp` (`self.DistanceAlongSpline`) 0.0 _returnvalue))
      (set `self.StopFollow` true))))

(fn `TakeOff`
  (locals (HasSetup :type Boolean) (AttachPointInputKey :type "Float (double-precision)"))
  (bind _atstation (`self.AtStation`))
  (if (not (`local.HasSetup`))
    (bind _output_get (set `local.AttachPointInputKey` (+ (`BlueprintMapLibrary.Map_Find` (`/Game/Blueprints/BP_Station.InputKeysOnLines` (`self.AtStation`)) (`self.CurrentLineIndex`)) (* 0.0 0.5))))
    (`/Game/Blueprints/BP_Station.SetTakeOffTrack` _atstation (`SplineComponent.GetLocationAtSplineInputKey` (`/Game/Blueprints/BP_Spline_Road.Spline` (`self.CurrentLine`)) _output_get "World"))
    (bind _output_get_2 (set `self.CurrentSpline` (`/Game/Blueprints/BP_Station.TakeOffTrack` _atstation)))
    (set `local.HasSetup` true))
  (`self.MoveAlongSpline` _output_get_2)
  (if (`self.StopFollow`)
    (`|ExecutionSequence`
      (:`then_0`
        (set `self.CurrentSpline` (`/Game/Blueprints/BP_Spline_Road.Spline` (`self.CurrentLine`))))
      (:`then_1`
        (set `self.DistanceAlongSpline` (`SplineComponent.GetDistanceAlongSplineAtSplineInputKey` (`self.CurrentSpline`) (`local.AttachPointInputKey`)))))))